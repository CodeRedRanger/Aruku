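; Actor component that runs branching NPC dialogue in a VR medical scenario, showing conversation nodes on the player pawn's menu.
; Choices adjust outcome and chaos scores, redirect the spouse's dialogue and trigger win, mixed, lose or chaos results in the game instance.
; Required actions (pulse check, AED retrieval or use, exam) pause dialogue on a pending node until completed, with AED retrieval gated by patient-area presence.
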(event `self.ReceiveBeginPlay`)

(fn `CompletePendingAction`
  (set `self.bWaitingForAction` false)
  (set `self.PendingAction` "NewEnumerator6")
  (set `self.CurrentConversationNodeID` (`self.PendingNodeID`))
  ; type in "None" ?
  (set `self.PendingNodeID` "None")
  ; already did in handle instruction ok clicked, but here too in case ok is not needed.
  (`/Game/VRTemplate/Blueprints/VRPawn.HideInstructionWidget` (`self.PlayerReference`))
  ;[1 0 0] show current node use branch? Because AED complete shouldn't  show current node
  (`/Game/VRTemplate/Blueprints/VRPawn.ShowConversationMenu` (`self.PlayerReference`) self))

(fn `FindConversationNode`
  (params (NodeToFind :type Name))
  (returns (FoundNode :type "/Game/EnumsStructs/ST_ConversationNode Structure") (Found :type Boolean))
  (locals (FoundLocal :type Boolean) (FoundNodeLocal :type "/Game/EnumsStructs/ST_ConversationNode Structure"))
  (set `local.FoundLocal` false)
  (for _array_element (`self.ConversationNodes`)
    (if (== (`.NodeID_2_F565E37D433812B048BD6DAE1147D862` (break `/Game/EnumsStructs/ST_ConversationNode` _array_element)) NodeToFind)
      (set `local.FoundLocal` true)
      (set `local.FoundNodeLocal` _array_element)
      (break)))
  (return (`local.FoundNodeLocal`) (`local.FoundLocal`)))

(fn `HandleAEDEnteredPatientArea`
  (set `self.bAEDInPatientArea` true)
  (if (`self.bWaitingForAction`)
    (if (`|EnumEquality` (`self.PendingAction`) "NewEnumerator1")
      (if (`self.bPlayerInPatientArea`)
        (`/Game/Actors/BP_AEDProcedure.SetUpAED` (`self.AEDProcedureRef`) null)
        (`self.CompletePendingAction`)))))

(fn `HandleConversationChoiceSelected`
  (params (ChoiceIndex :type Integer))
  (bind _gameinstanceref (`self.GameInstanceRef`))
  (bind _gameinstanceref_2 (`self.GameInstanceRef`))
  (bind _gameinstanceref_3 (`self.GameInstanceRef`))
  (bind _gameinstanceref_4 (`self.GameInstanceRef`))
  (bind _bppatientspouseref (`/Game/VRTemplate/Blueprints/VRPawn.BPPatientSpouseRef` (`self.PlayerReference`)))
  (bind _bppatientspouseref_2 (`/Game/VRTemplate/Blueprints/VRPawn.BPPatientSpouseRef` (`self.PlayerReference`)))
  (bind _bp_conversationcomponent (`/Game/Actors/BP_PatientSpouse.BP_ConversationComponent` _bppatientspouseref_2))
  (bind (_choicetext _nextnodeid _outcomechange _chaoschange _endconversation _triggerswin _triggerslose _requiredaction) (break `/Game/EnumsStructs/ST_ConversationChoice` (`|GetArrayItem` (`.Choices_9_D0451EF347A3275670A23C85A16A1F46` (break `/Game/EnumsStructs/ST_ConversationNode` (`self.CurrentNodeData`))) ChoiceIndex)))
  (bind _returnvalue (`|EnumEquality` _requiredaction "NewEnumerator6"))
  ; handle spouse answer
  (if (`KismetArrayLibrary.Array_IsValidIndex` (`.Choices_9_D0451EF347A3275670A23C85A16A1F46` (break `/Game/EnumsStructs/ST_ConversationNode` (`self.CurrentNodeData`))) ChoiceIndex)
    (if (and (== (`self.CurrentConversationNodeID`) (`/Game/VRTemplate/Blueprints/VRPawn.SpouseTriggerNodeID` (`self.PlayerReference`))) (not (`/Game/VRTemplate/Blueprints/VRPawn.bSpokeWithSpouse` (`self.PlayerReference`))))
      (set `/Game/VRTemplate/Blueprints/VRPawn.bSpokeWithSpouse` true (`self.PlayerReference`))
      (elif (> _outcomechange 0.0)
        (set `/Game/Utility/BP_ConversationComponent.StartingNodeID` (`/Game/Actors/BP_PatientSpouse.SpouseImproveNodeID` _bppatientspouseref_2) _bp_conversationcomponent)
        (elif (< _outcomechange 0.0)
          (set `/Game/Utility/BP_ConversationComponent.StartingNodeID` (`/Game/Actors/BP_PatientSpouse.SpouseWorseNodeID` _bppatientspouseref_2) _bp_conversationcomponent))))
    ; C++
    (bind _returnvalue_2 (`self.CalculateChaosScore` _chaoschange))
    (if (>= _returnvalue_2 50.0)
      (set `/Game/Utility/BP_ConversationComponent.StartingNodeID` (`/Game/Actors/BP_PatientSpouse.SpouseChaosNodeID` _bppatientspouseref) (`/Game/Actors/BP_PatientSpouse.BP_ConversationComponent` _bppatientspouseref)))
    (bind _asbp_med_game_instance (cast `/Game/Utility/BP_MedGameInstance` (`GameplayStatics.GetGameInstance`)))
    (bind _output_get (set `self.GameInstanceRef` _asbp_med_game_instance))
    (bind _output_get_2 (set `/Game/Utility/BP_MedGameInstance.OutcomeScore` (`KismetMathLibrary.FClamp` (+ _outcomechange (`/Game/Utility/BP_MedGameInstance.OutcomeScore` _asbp_med_game_instance)) 0.0 100.0) _output_get))
    (`self.UpdateOutcomeMeter` _output_get_2)
    ; lose branch is first
    (if _triggerslose
      (`/Game/VRTemplate/Blueprints/VRPawn.CloseConversationMenu` (`self.PlayerReference`) :!label _label)
      (`/Game/Utility/BP_MedGameInstance.SetScenarioResult` _gameinstanceref_2 "NewEnumerator1" (`/Game/Utility/BP_MedGameInstance.LoseResultTitle` _gameinstanceref_2) (`/Game/Utility/BP_MedGameInstance.LoseResultMessage` _gameinstanceref_2) _output_get_2 "VRTemplateMap" "None")
      (set `/Game/Utility/BP_MedGameInstance.OutcomeScore` 50.0 (`self.GameInstanceRef`))
      ; C++
      (`self.RespondToChaos` _returnvalue_2 true)
      (elif (and _triggerswin (< _output_get_2 60.0))
        (goto _label)
        (elif (and _triggerswin (>= _output_get_2 60.0) (< _output_get_2 75.0))
          (`/Game/Utility/BP_MedGameInstance.SetScenarioResult` _gameinstanceref_3 "NewEnumerator2" (`/Game/Utility/BP_MedGameInstance.MixedResultTitle` _gameinstanceref_3) (`/Game/Utility/BP_MedGameInstance.MixedResultMessage` _gameinstanceref_3) _output_get_2 "VRTemplateMap" "None")
          (set `/Game/Utility/BP_MedGameInstance.OutcomeScore` 50.0 (`self.GameInstanceRef`))
          ; C++
          (`self.RespondToChaos` _returnvalue_2 true)
          (else
            ; win branch
            (if (and _triggerswin (>= _output_get_2 75.0))
              (`/Game/VRTemplate/Blueprints/VRPawn.CloseConversationMenu` (`self.PlayerReference`))
              (`/Game/Utility/BP_MedGameInstance.SetScenarioResult` _gameinstanceref_4 "NewEnumerator0" (`/Game/Utility/BP_MedGameInstance.WinResultTitle` _gameinstanceref_4) (`/Game/Utility/BP_MedGameInstance.WinResultMessage` _gameinstanceref_4) _output_get_2 "VRTemplateMap" "None")
              (set `/Game/Utility/BP_MedGameInstance.OutcomeScore` 50.0 (`self.GameInstanceRef`))
              ; C++
              (`self.RespondToChaos` _returnvalue_2 true)
              (else
                ; C++ function
                (`self.RespondToChaos` _returnvalue_2)
                (if (>= _returnvalue_2 80.0)
                  (`/Game/VRTemplate/Blueprints/VRPawn.CloseConversationMenu` (`self.PlayerReference`))
                  (`/Game/Utility/BP_MedGameInstance.SetScenarioResult` _gameinstanceref "NewEnumerator3" (`/Game/Utility/BP_MedGameInstance.ChaosResultTitle` _gameinstanceref) (`/Game/Utility/BP_MedGameInstance.ChaosResultMessage` _gameinstanceref) _output_get_2 "VRTemplateMap" "None")
                  (set `/Game/Utility/BP_MedGameInstance.OutcomeScore` 50.0 (`self.GameInstanceRef`))
                  (`self.RespondToChaos` 0.0 true)
                  (else
                    ; end conversation branch
                    (if _endconversation
                      (if _returnvalue
                        ; So you can start where you left off
                        (set `self.StartingNodeID` (`self.CurrentConversationNodeID`))
                        (`/Game/VRTemplate/Blueprints/VRPawn.CloseConversationMenu` (`self.PlayerReference`))
                        (else
                          (switch `/Game/EnumsStructs/EConversationAction` _requiredaction :!label _label_2
                            (:`NewEnumerator0`
                              (`self.HandleRequiredActionCheckPulse` _nextnodeid)
                              (`/Engine/EditorBlueprintResources/StandardMacros.IsValid` (`self.CarotidPulseProcedureRef`)
                                (:`Is Valid`
                                  (`/Game/Actors/BP_CarotidPulseProcedure.StartProcedure` (`self.CarotidPulseProcedureRef`) self))
                                (:`Is Not Valid`
                                  (`KismetSystemLibrary.PrintString` "Carotid Procedure reference was not assigned" true true (struct :`G` 0.66 :`B` 1.0 :`A` 1.0) 10.0))))
                            (:`NewEnumerator1`
                              (`self.HandleRequiredActionRetrieveAED` _nextnodeid))
                            (:`NewEnumerator7`
                              (`self.HandleRequiredActionUseAED` _nextnodeid)
                              (`/Engine/EditorBlueprintResources/StandardMacros.IsValid` (`self.AEDProcedureRef`)
                                (:`Is Valid`
                                  (`/Game/Actors/BP_AEDProcedure.StartProcedure` (`self.AEDProcedureRef`) self))
                                (:`Is Not Valid`
                                  (`KismetSystemLibrary.PrintString` "AED Procedure reference was not assigned" true true (struct :`G` 0.66 :`B` 1.0 :`A` 1.0) 10.0))))
                            (:`NewEnumerator10`
                              (`self.HandleRequiredActionPerformExam` _nextnodeid)
                              (`/Engine/EditorBlueprintResources/StandardMacros.IsValid` (`self.ExamProcedureRef`)
                                (:`Is Valid`
                                  (`/Game/Actors/BP_ExamProcedure.StartProcedure` (`self.ExamProcedureRef`) self))
                                (:`Is Not Valid`
                                  (`KismetSystemLibrary.PrintString` "Exam Procedure reference was not assigned" true true (struct :`G` 0.66 :`B` 1.0 :`A` 1.0) 10.0)))))))
                      (elif _returnvalue
                        (set `self.CurrentConversationNodeID` _nextnodeid)
                        (`self.ShowCurrentNode`)
                        (else
                          (goto _label_2))))))))))))
    (else
      (`KismetSystemLibrary.PrintString` "Invalid conversation choice index"))))

(fn `HandlePlayerEnteredPatientArea`
  (set `self.bPlayerInPatientArea` true)
  (if (`self.bWaitingForAction`)
    (if (`|EnumEquality` (`self.PendingAction`) "NewEnumerator1")
      (if (`self.bAEDInPatientArea`)
        ;[0.5 0.05 0.05] need to create content of this function, should go on to talk prompt
        (`self.CompletePendingAction`)
        (else
          (`/Game/VRTemplate/Blueprints/VRPawn.ShowConversationInstruction` (`self.PlayerReference`) (`/Game/Actors/BP_AEDProcedure.AEDMissingInstructionText` (`self.AEDProcedureRef`)) true true ""))))))

(fn `HandlePlayerLeftPatientArea`
  (set `self.bPlayerInPatientArea` false))

(fn `HandleRequiredActionCheckPulse`
  (params (NextNodeID :type Name))
  (set `self.PendingAction` "NewEnumerator0")
  (if (== NextNodeID "None")
    (`KismetSystemLibrary.PrintString` "ERROR: Action choice has no NextNodeID" true true (struct :`R` 0.5 :`G` 0.05 :`B` 0.05 :`A` 1.0) 10.0)
    (else
      (set `self.PendingNodeID` NextNodeID)
      (set `self.bWaitingForAction` true)
      (`/Game/VRTemplate/Blueprints/VRPawn.CloseConversationMenu` (`self.PlayerReference`)))))

(fn `HandleRequiredActionPerformExam`
  (params (NextNodeID :type Name))
  (set `self.PendingAction` "NewEnumerator10")
  (if (== NextNodeID "None")
    (`KismetSystemLibrary.PrintString` "ERROR: Action choice has no NextNodeID" true true (struct :`R` 0.5 :`G` 0.05 :`B` 0.05 :`A` 1.0) 10.0)
    (else
      (set `self.PendingNodeID` NextNodeID)
      (set `self.bWaitingForAction` true)
      (`/Game/VRTemplate/Blueprints/VRPawn.CloseConversationMenu` (`self.PlayerReference`)))))

(fn `HandleRequiredActionRetrieveAED`
  (params (NextNodeID :type Name))
  (set `self.PendingAction` "NewEnumerator1")
  (if (== NextNodeID "None")
    (`KismetSystemLibrary.PrintString` "ERROR: Action choice has no NextNodeID" true true (struct :`R` 0.5 :`G` 0.05 :`B` 0.05 :`A` 1.0) 10.0)
    (else
      (set `self.PendingNodeID` NextNodeID)
      (set `self.bWaitingForAction` true)
      (`/Game/VRTemplate/Blueprints/VRPawn.CloseConversationMenu` (`self.PlayerReference`))
      (if (`PrimitiveComponent.IsOverlappingActor` (`/Game/Actors/BP_Patient.InteractionRange` (`/Game/VRTemplate/Blueprints/VRPawn.BPPatientRef` (`self.PlayerReference`))) (`/Game/Actors/BP_AEDProcedure.BPAEDRef` (`self.AEDProcedureRef`)))
        (`/Game/Actors/BP_AEDProcedure.SetUpAED` (`self.AEDProcedureRef`) null)
        (`self.CompletePendingAction`)))))

(fn `HandleRequiredActionUseAED`
  (params (NextNodeID :type Name))
  (set `self.PendingAction` "NewEnumerator7")
  (if (== NextNodeID "None")
    (`KismetSystemLibrary.PrintString` "ERROR: Action choice has no NextNodeID" true true (struct :`R` 0.5 :`G` 0.05 :`B` 0.05 :`A` 1.0) 10.0)
    (else
      (set `self.PendingNodeID` NextNodeID)
      (set `self.bWaitingForAction` true)
      (`/Game/VRTemplate/Blueprints/VRPawn.CloseConversationMenu` (`self.PlayerReference`)))))

(fn `ShowCurrentNode`
  (`|ExecutionSequence`
    (:`then_0`
      (if (== (`self.CurrentConversationNodeID`) "ChestPainStart")
        (`GameplayStatics.PlaySound2D` "/Game/Assets/Audio/SFX/pain.pain" (`/Game/Utility/BP_MedGameInstance.SavedSFXVolume` (`self.GameInstanceRef`)) 1.0 0.0 null null)))
    (:`then_1`
      (if (== (`self.CurrentConversationNodeID`) "PatientUnresponsiveStartSpouse")
        (`AudioComponent.Play` (`NPCStatic.NPCReactionAudioComponent` (`/Game/VRTemplate/Blueprints/VRPawn.BPPatientSpouseRef` (`self.PlayerReference`))) 0.0)))
    (:`then_2`
      (bind (_foundnode _found) (`self.FindConversationNode` (`self.CurrentConversationNodeID`)))
      (if _found
        (bind _output_get (set `self.CurrentNodeData` _foundnode))
        (`/Engine/EditorBlueprintResources/StandardMacros.IsValid` (`self.PlayerReference`)
          (:`Is Valid`
            (`/Game/VRTemplate/Blueprints/VRPawn.DisplayConversationNode` (`self.PlayerReference`) _output_get)))
        (else
          (`KismetSystemLibrary.PrintString` "Conversation node not found: [CurrentConversationNodeID]" true true (struct :`R` 0.5 :`G` 0.05 :`B` 0.05 :`A` 1.0) 20.0))))))

(fn `StartConversation`
  (set `self.CurrentConversationNodeID` (`self.StartingNodeID`))
  (bind _asvrpawn (cast `/Game/VRTemplate/Blueprints/VRPawn` (`GameplayStatics.GetPlayerPawn` 0)))
  (bind _output_get (set `self.PlayerReference` _asvrpawn))
  (`/Game/VRTemplate/Blueprints/VRPawn.ShowConversationMenu` _output_get self))

(fn `UpdateOutcomeMeter`
  (params (OutcomeValue :type "Float (double-precision)"))
  (bind _asbp_patient (cast `/Game/Actors/BP_Patient` (`self.GetOwner`)))
  (bind _aswbp_outcome_meter (cast `/Game/Widgets/WBP_OutcomeMeter` (`WidgetComponent.GetUserWidgetObject` (`/Game/Actors/BP_Patient.OutcomeMeterWidget` _asbp_patient))))
  (`/Game/Widgets/WBP_OutcomeMeter.SetOutcomeValue` _aswbp_outcome_meter OutcomeValue))