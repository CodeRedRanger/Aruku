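; Game instance for a VR scenario game that holds persistent settings, scenario results and multiplayer network state across levels.
; On Init it loads the settings save, then applies volumes through a sound mix and quality through console commands.
; Scenario results play applause or booing, save a new high score and open the pawn's result menu.
; It also handles level loading, network failure and leave states, and shared UI sounds.
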(event `self.ReceiveInit`
  (`self.LoadSettings`))

(event `self.ResetNetworkStateForLeave`
  (set `self.NetworkState` "NewEnumerator0")
  ; Should reset the multiplayer menu options
  (set `self.SavedNetworkOption` "NewEnumerator0"))

(event `self.HandleNetworkFailureState`
  (params (ErrorMessage :type String))
  (bind _aswbp_multiplayer_options (cast `/Game/Widgets/WBP_MultiplayerOptions` (`WidgetComponent.GetUserWidgetObject` (`/Game/VRTemplate/Blueprints/VRPawn.MultiplayerOptionsWidget` (`self.VRPawn`)))))
  (switch `/Game/EnumsStructs/ENetworkMenuOption` (`/Game/Widgets/WBP_MultiplayerOptions.SelectedNetworkOption` _aswbp_multiplayer_options)
    (:`NewEnumerator2`
      (set `self.NetworkState` "NewEnumerator4")
      (bind _output_get (set `/Game/Widgets/WBP_MultiplayerOptions.SelectedNetworkOption` "NewEnumerator0" _aswbp_multiplayer_options))
      (set `self.SavedNetworkOption` _output_get))
    (:`NewEnumerator6`
      (`/Game/Widgets/WBP_MultiplayerOptions.OnNetworkFailed` _aswbp_multiplayer_options)
      (set `self.NetworkState` "NewEnumerator8")
      (bind _output_get_2 (set `/Game/Widgets/WBP_MultiplayerOptions.SelectedNetworkOption` "NewEnumerator2" _aswbp_multiplayer_options))
      (set `self.SavedNetworkOption` _output_get_2))))

(fn `ApplyAudioSettings`
  (`GameplayStatics.PushSoundMixModifier` "/Game/Assets/Audio/SM_Settings.SM_Settings")
  (if (`self.SavedMasterMuted`)
    (set `self.SavedMasterVolume` 0.0)
    (set `self.CurrentMasterVolume` 0.0)
    (else
      (set `self.CurrentMasterVolume` (`self.SavedMasterVolume`))))
  (if (`self.SavedMusicMuted`)
    (set `self.SavedMusicVolume` 0.0)
    (set `self.CurrentMusicVolume` 0.0)
    (else
      (set `self.CurrentMusicVolume` (`self.SavedMusicVolume`))))
  (if (`self.SavedSFXMuted`)
    (set `self.SavedSFXVolume` 0.0)
    (set `self.CurrentSFXVolume` 0.0)
    (else
      (set `self.CurrentSFXVolume` (`self.SavedSFXVolume`))))
  (`GameplayStatics.SetSoundMixClassOverride` "/Game/Assets/Audio/SM_Settings.SM_Settings" "/Game/Assets/Audio/SoundClasses/SC_Master.SC_Master" (`self.CurrentMasterVolume`))
  (`GameplayStatics.SetSoundMixClassOverride` "/Game/Assets/Audio/SM_Settings.SM_Settings" "/Game/Assets/Audio/SoundClasses/SC_Music.SC_Music" (`self.CurrentMusicVolume`))
  (`GameplayStatics.SetSoundMixClassOverride` "/Game/Assets/Audio/SM_Settings.SM_Settings" "/Game/Assets/Audio/SoundClasses/SC_SFX.SC_SFX" (`self.CurrentSFXVolume`))
  ; Restarts pause music if mute apply and then unmute apply on pause screen
  (bind _asvrpawn (cast `/Game/VRTemplate/Blueprints/VRPawn` (`GameplayStatics.GetPlayerPawn` 0)))
  (set `self.VRPawn` _asvrpawn)
  (if (and (`KismetMathLibrary.BooleanNOR` (`self.SavedMasterMuted`) (`self.SavedMusicMuted`)) (> (`self.CurrentMusicVolume`) 0.0))
    (if (and (`|EnumEquality` (`/Game/VRTemplate/Blueprints/VRPawn.ActiveMenuState` (`self.VRPawn`)) "NewEnumerator4") (not (`self.LoadingMainMenu`)))
      (`AudioComponent.Play` (`/Game/VRTemplate/Blueprints/VRPawn.PawnAudioCompOptions` (`self.VRPawn`)) 0.0)
      (elif (`|EnumEquality` (`/Game/VRTemplate/Blueprints/VRPawn.ActiveMenuState` (`self.VRPawn`)) "NewEnumerator6")
        (`AudioComponent.Play` (`/Game/Actors/BP_MainMenuPanel.OptionsMenuAudioCompRef` (`self.MainMenuPanelRef`)) 0.0)))))

(fn `ApplyGraphicsSettings`
  (switch `/Game/EnumsStructs/EGraphicsQuality` (`self.SavedGraphicsQuality`)
    (:`NewEnumerator0`
      (`KismetSystemLibrary.ExecuteConsoleCommand` "sg.SetQuality 0" null))
    (:`NewEnumerator1`
      (`KismetSystemLibrary.ExecuteConsoleCommand` "sg.SetQuality 1" null))
    (:`NewEnumerator2`
      (`KismetSystemLibrary.ExecuteConsoleCommand` "sg.SetQuality 2" null))
    (:`NewEnumerator3`
      (`KismetSystemLibrary.ExecuteConsoleCommand` "sg.SetQuality 3" null)))
  (switch `/Game/EnumsStructs/ERenderQuality` (`self.SavedVRRenderQuality`)
    (:`NewEnumerator0`
      (`KismetSystemLibrary.ExecuteConsoleCommand` "xr.SecondaryScreenPercentage.HMDRenderTarget 70" null))
    (:`NewEnumerator1`
      (`KismetSystemLibrary.ExecuteConsoleCommand` "xr.SecondaryScreenPercentage.HMDRenderTarget 100" null))
    (:`NewEnumerator2`
      (`KismetSystemLibrary.ExecuteConsoleCommand` "xr.SecondaryScreenPercentage.HMDRenderTarget 120" null))))

(fn `LoadFirstScenario`
  (set `self.CurrentScenarioLevel` (`self.FirstScenarioLevel`))
  (`GameplayStatics.OpenLevel` (`self.FirstScenarioLevel`)))

(fn `LoadMainMenu`
  (switch `/Game/EnumsStructs/ENetworkMenuOption` (`self.NetworkState`)
    (:`NewEnumerator0`
      (set `self.LoadingMainMenu` true)
      (set `self.CurrentScenarioLevel` (`self.MainMenuLevel`))
      (`GameplayStatics.OpenLevel` (`self.MainMenuLevel`)))
    (:`NewEnumerator1`
      (`self.LeaveNetworkGame` :!label _label))
    (:`NewEnumerator2`
      (goto _label))))

(fn `LoadNextScenario`
  (`GameplayStatics.OpenLevel` (`self.MainMenuLevel`)))

(fn `LoadSettings`
  (bind _settingsuserindex (`self.SettingsUserIndex`))
  (bind _settingsslotname (`self.SettingsSlotName`))
  (bind _returnvalue (`GameplayStatics.DoesSaveGameExist` _settingsslotname _settingsuserindex))
  (if _returnvalue
    (bind _returnvalue_2 (`GameplayStatics.LoadGameFromSlot` _settingsslotname _settingsuserindex))
    (bind _assg_game_settings (cast `/Game/Utility/SG_GameSettings` _returnvalue_2))
    (set `self.SG Game Settings` _assg_game_settings)
    (set `self.SavedMasterVolume` (`/Game/Utility/SG_GameSettings.MasterVolume` (`self.SG Game Settings`)))
    (set `self.SavedMusicVolume` (`/Game/Utility/SG_GameSettings.MusicVolume` (`self.SG Game Settings`)))
    (set `self.SavedSFXVolume` (`/Game/Utility/SG_GameSettings.SFXVolume` (`self.SG Game Settings`)))
    (set `self.SavedMasterMuted` (`/Game/Utility/SG_GameSettings.MasterMute` (`self.SG Game Settings`)))
    (set `self.SavedMusicMuted` (`/Game/Utility/SG_GameSettings.MusicMute` (`self.SG Game Settings`)))
    (set `self.SavedSFXMuted` (`/Game/Utility/SG_GameSettings.SFXMute` (`self.SG Game Settings`)))
    (set `self.SavedGraphicsQuality` (`/Game/Utility/SG_GameSettings.GraphicsQuality` (`self.SG Game Settings`)))
    (set `self.SavedVRRenderQuality` (`/Game/Utility/SG_GameSettings.VRRenderQuality` (`self.SG Game Settings`)))
    (`self.ApplyAudioSettings`)
    (`self.ApplyGraphicsSettings`)
    (set `self.SavedHighScoreLevel1` (`/Game/Utility/SG_GameSettings.HighScoreLevel1` (`self.SG Game Settings`)))
    (else
      (`self.ApplyAudioSettings`)
      (`self.ApplyGraphicsSettings`)
      (`self.SaveSettings`))))

(fn `PlayButtonClick`
  (`/Engine/EditorBlueprintResources/StandardMacros.IsValid` (`self.ButtonClickedSound`)
    (:`Is Valid`
      (`GameplayStatics.PlaySound2D` (`self.ButtonClickedSound`) 1.0 1.0 0.0 null null))))

(fn `PlayButtonHover`
  (`/Engine/EditorBlueprintResources/StandardMacros.IsValid` (`self.ButtonHoverSound`)
    (:`Is Valid`
      (`GameplayStatics.PlaySound2D` (`self.ButtonHoverSound`) 1.0 1.0 0.0 null null))))

(fn `PlayErrorSound`
  (`/Engine/EditorBlueprintResources/StandardMacros.IsValid` (`self.ErrorSound`)
    (:`Is Valid`
      (`GameplayStatics.PlaySound2D` (`self.ErrorSound`) 1.0 1.0 0.0 null null))))

(fn `PlayMenuClose`
  (`/Engine/EditorBlueprintResources/StandardMacros.IsValid` (`self.MenuCloseSound`)
    (:`Is Valid`
      (`GameplayStatics.PlaySound2D` (`self.MenuCloseSound`) 1.0 1.0 0.0 null null))))

(fn `PlayMenuOpen`
  (`/Engine/EditorBlueprintResources/StandardMacros.IsValid` (`self.MenuOpenSound`)
    (:`Is Valid`
      (`GameplayStatics.PlaySound2D` (`self.MenuOpenSound`) 1.0 1.0 0.0 null null))))

(fn `QuitGame`)

(fn `ReplayCurrentScenario`
  (`GameplayStatics.OpenLevel` (`self.CurrentScenarioLevel`))
  (set `self.OutcomeScore` 50.0)
  (`/Engine/EditorBlueprintResources/StandardMacros.IsValid` (`/Game/VRTemplate/Blueprints/VRPawn.ActiveConversationComponent` (`self.VRPawn`))
    (:`Is Valid`
      ; Stops the crowd noise, chaos score reset in pawn begin play (could reset outcome there too)
      (`ConversationComponent.RespondToChaos` (`/Game/VRTemplate/Blueprints/VRPawn.ActiveConversationComponent` (`self.VRPawn`)) 0.0 true))))

(fn `ResumeCurrentScenario`
  (bind _asvrpawn (cast `/Game/VRTemplate/Blueprints/VRPawn` (`GameplayStatics.GetPlayerPawn` 0)))
  (`/Game/VRTemplate/Blueprints/VRPawn.TogglePauseMenu` _asvrpawn))

(fn `SaveSettings`
  (bind _returnvalue (`GameplayStatics.CreateSaveGameObject` "/Game/Utility/SG_GameSettings.SG_GameSettings_C"))
  (bind _assg_game_settings (cast `/Game/Utility/SG_GameSettings` _returnvalue))
  (bind _output_get (set `self.SG Game Settings` _assg_game_settings))
  (set `/Game/Utility/SG_GameSettings.MasterVolume` (`self.SavedMasterVolume`) _output_get)
  (set `/Game/Utility/SG_GameSettings.MusicVolume` (`self.SavedMusicVolume`) (`self.SG Game Settings`))
  (set `/Game/Utility/SG_GameSettings.SFXVolume` (`self.SavedSFXVolume`) (`self.SG Game Settings`))
  (set `/Game/Utility/SG_GameSettings.MasterMute` (`self.SavedMasterMuted`) (`self.SG Game Settings`))
  (set `/Game/Utility/SG_GameSettings.MusicMute` (`self.SavedMusicMuted`) (`self.SG Game Settings`))
  (set `/Game/Utility/SG_GameSettings.SFXMute` (`self.SavedSFXMuted`) (`self.SG Game Settings`))
  (set `/Game/Utility/SG_GameSettings.GraphicsQuality` (`self.SavedGraphicsQuality`) (`self.SG Game Settings`))
  (set `/Game/Utility/SG_GameSettings.VRRenderQuality` (`self.SavedVRRenderQuality`) (`self.SG Game Settings`))
  ; Later make a loop that saves all high scores and ssave high scores into an array of floats in both SG and GI classes
  (set `/Game/Utility/SG_GameSettings.HighScoreLevel1` (`self.SavedHighScoreLevel1`) (`self.SG Game Settings`))
  (`GameplayStatics.SaveGameToSlot` (`self.SG Game Settings`) (`self.SettingsSlotName`) (`self.SettingsUserIndex`)))

(fn `SetScenarioResult`
  (params (NewResultType :type "/Game/EnumsStructs/EGameResult Enum" :default "NewEnumerator0") (NewResultTitle :type Text) (NewResultMessage :type Text) (NewOutcomeScore :type "Float (double-precision)") (NewCurrentScenarioLevel :type Name) (NewNextScenarioLevel :type Name))
  (if (`|EnumEquality` NewResultType "NewEnumerator0")
    (`GameplayStatics.PlaySound2D` "/Game/Assets/Audio/SFX/applause.applause" 1.0 1.0 0.0 null null)
    (else
      (`GameplayStatics.PlaySound2D` "/Game/Assets/Audio/SFX/booing.booing" 1.0 1.0 0.0 null null)))
  (set `self.ResultType` NewResultType)
  (set `self.ResultTitle` NewResultTitle)
  (set `self.ResultMessage` NewResultMessage)
  (set `self.OutcomeScore` NewOutcomeScore)
  (set `self.CurrentScenarioLevel` NewCurrentScenarioLevel)
  (set `self.NextScenarioLevel` NewNextScenarioLevel)
  (`self.ShowResultsMenuPawn`))

(fn `ShowResultsMenuPawn`
  (if (> (`self.OutcomeScore`) (`self.SavedHighScoreLevel1`))
    (set `self.SavedHighScoreLevel1` (`self.OutcomeScore`))
    (`self.SaveSettings`))
  (bind _asvrpawn (cast `/Game/VRTemplate/Blueprints/VRPawn` (`GameplayStatics.GetPlayerPawn` 0)))
  (`/Game/VRTemplate/Blueprints/VRPawn.ShowResultMenu` _asvrpawn))