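; Flight attendant AI character that walks up to the VR player and opens the intro dialog.
; On BeginPlay it registers itself with the VRPawn, then moves to a point StopDistance short of the player along the line between them.
; On arrival, FacePlayer interpolates yaw toward the VR camera and disables orient-to-movement before the pawn shows the dialog.
; Tick repeats that turn while ShouldFacePlayer is true, which nothing here sets.
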(event `self.ReceiveBeginPlay`
  (`parent.ReceiveBeginPlay`)
  (bind _asvrpawn (cast `/Game/VRTemplate/Blueprints/VRPawn` (`GameplayStatics.GetPlayerPawn` 0))
    (:`then`
      (set `self.PlayerReference` _asvrpawn)
      (set `/Game/VRTemplate/Blueprints/VRPawn.BPFlightAttendantReference` self _asvrpawn)
      (bind _returnvalue (`self.CalculateApproachLocation` (`self.PlayerReference`)))
      (`|AIMoveTo` self _returnvalue null 150.0
        (:`OnSuccess`
          (bind _asvrpawn_2 (`self.FacePlayer`))
          (`/Game/VRTemplate/Blueprints/VRPawn.ShowIntroDialog` _asvrpawn_2))
        (:`OnFail`
          (`KismetSystemLibrary.PrintString` "Flight attendant failed to move" true true (struct :`G` 0.66 :`B` 1.0 :`A` 1.0) 10.0))))
    (:`CastFailed`
      (`KismetSystemLibrary.PrintString` "failed to cast to vr pawn" true true (struct :`G` 0.66 :`B` 1.0 :`A` 1.0) 20.0))))

(event `self.ReceiveTick`
  (params (DeltaSeconds :type "Float (single-precision)"))
  (`parent.ReceiveTick` DeltaSeconds)
  (if (`self.bShouldFacePlayer`)
    (`self.FacePlayer`)))

(fn `CalculateApproachLocation`
  (params (DestinationActor :type "Actor Object Reference"))
  (returns (ReturnValue :type "Vector Structure"))
  (bind _returnvalue (`self.K2_GetActorLocation` DestinationActor))
  (return (+ _returnvalue (* (`KismetMathLibrary.Normal` (- (`self.K2_GetActorLocation`) _returnvalue)) (`self.StopDistance`)))))

(fn `FacePlayer`
  (returns (AsVRPawn :type "/Game/VRTemplate/Blueprints/VRPawn Object Reference"))
  (bind (_returnvalue_roll _returnvalue_pitch _returnvalue_yaw) (`KismetMathLibrary.BreakRotator` (`self.K2_GetActorRotation`)))
  (bind _asvrpawn (cast `/Game/VRTemplate/Blueprints/VRPawn` (`GameplayStatics.GetPlayerPawn` 0))
    (:`then`
      (bind (_returnvalue_roll_2 _returnvalue_pitch_2 _returnvalue_yaw_2) (`KismetMathLibrary.BreakRotator` (`KismetMathLibrary.FindLookAtRotation` (`self.K2_GetActorLocation`) (`SceneComponent.K2_GetComponentLocation` (`/Game/VRTemplate/Blueprints/VRPawn.Camera` _asvrpawn)))))
      (bind (_returnvalue_roll_3 _returnvalue_pitch_3 _returnvalue_yaw_3) (`KismetMathLibrary.BreakRotator` (`KismetMathLibrary.RInterpTo` (`KismetMathLibrary.MakeRotator` 0.0 0.0 _returnvalue_yaw) (`KismetMathLibrary.MakeRotator` 0.0 0.0 _returnvalue_yaw_2) (`GameplayStatics.GetWorldDeltaSeconds`) 4.0)))
      (`self.K2_SetActorRotation` (`KismetMathLibrary.MakeRotator` 0.0 0.0 _returnvalue_yaw_3))
      (set `CharacterMovementComponent.bOrientRotationToMovement` false (`self.CharacterMovement`)))
    (:`CastFailed`
      _))
  (return _asvrpawn))

(fn `UserConstructionScript`
  (`parent.UserConstructionScript`))