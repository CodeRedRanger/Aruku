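; BP_AEDPad is a grabbable AED pad actor for VR that can be returned to a stored home transform.
; ResetPad makes the player's VRPawn force-release its held object, detaches the pad, zeroes its linear and angular velocity, disables physics and teleports it to HomeTransform.
; The teleport relies on the static mesh being the root component.
; Event graph and construction script hold no logic.
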(fn `ResetPad`
  (bind _asvrpawn (cast `/Game/VRTemplate/Blueprints/VRPawn` (`GameplayStatics.GetPlayerPawn` 0)))
  (`/Game/VRTemplate/Blueprints/VRPawn.ForceReleaseObject` _asvrpawn)
  (`self.K2_DetachFromActor` "KeepWorld" "KeepWorld" "KeepWorld")
  (`PrimitiveComponent.SetPhysicsLinearVelocity` (`self.StaticMesh`) (0.0 0.0 0.0) false "None")
  (`PrimitiveComponent.SetPhysicsAngularVelocityInDegrees` (`self.StaticMesh`) (0.0 0.0 0.0) false "None")
  (`PrimitiveComponent.SetSimulatePhysics` (`self.StaticMesh`) false)
  ; works because mesh is root
  (`self.K2_SetActorTransform` (`self.HomeTransform`) false true)
  (`PrimitiveComponent.SetSimulatePhysics` (`self.StaticMesh`) false))

(fn `UserConstructionScript`)