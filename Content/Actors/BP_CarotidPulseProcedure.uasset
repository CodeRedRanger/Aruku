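; VR carotid pulse check procedure, where the player picks the pulse site on an enlarged patient that replaces the normal one.
; Five WBP_CarotidTarget widgets with IDs report to HandleTargetSelected, which shows feedback through the pawn's instruction widget and plays heartbeat or booing audio.
; EndProcedure restores the patient and completes the conversation component's pending action.
; RestoreProcedureDisplay re-applies prompt and button state; pad-placement functions are inert.
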(event `self.ReceiveBeginPlay`
  (`self.InitializeTargetWidgets`)
  (bind _asvrpawn (cast `/Game/VRTemplate/Blueprints/VRPawn` (`GameplayStatics.GetPlayerPawn` 0)))
  (set `self.VRPawnRef` _asvrpawn)
  (bind _aswbp_instruction (cast `/Game/Widgets/WBP_Instruction` (`WidgetComponent.GetUserWidgetObject` (`/Game/VRTemplate/Blueprints/VRPawn.InstructionWidget` (`self.VRPawnRef`)))))
  (bind _output_get (set `self.InstructionWidgetRef` _aswbp_instruction))
  (add `/Game/Widgets/WBP_Instruction.OnInstructionOKButtonClicked` _output_get (`|CreateDelegate` (`self.VRPawnRef`) :!event `HandleInstructionOKClicked`))
  (`self.SetAllTargetInteractionEnabled` false)
  (`self.ShowHideAllTargets` true)
  ;[1 0 0] disable the AED pad collision areas if needed (check if touching area causes aed pad feedback sounds)
  (`/Game/Actors/BP_EnlargedPatient.HideEnlargedPatient` (`self.BPEnlargedPatientRef`))
  (set `/Game/Actors/BP_EnlargedPatient.CarotidPulseProcedureRef` self (`self.BPEnlargedPatientRef`))
  (bind _aswbp_carotid_target (cast `/Game/Widgets/WBP_CarotidTarget` (`WidgetComponent.GetUserWidgetObject` (`self.CarotidTarget_Left`))))
  (set `/Game/Widgets/WBP_CarotidTarget.ProcedureReference` self _aswbp_carotid_target))

(fn `CompleteBackPadPlacement`
  (params (PadReference :type "/Game/Actors/BP_AEDPad Object Reference"))
  (locals (CurrentPad :type "/Game/Actors/BP_AEDPad Object Reference")))

(fn `CompleteFrontPadPlacement`
  (params (PadReference :type "/Game/Actors/BP_AEDPad Object Reference"))
  (locals (CurrentPad :type "/Game/Actors/BP_AEDPad Object Reference")))

(fn `EndProcedure`
  ;[1 0 0] Could hide instruction menu here instead handle click ok in pawn. Also done in complete pending action
  ;; Must hide target widgets too
  (`self.SetAllTargetInteractionEnabled` false)
  (`self.ShowHideAllTargets` true)
  (`SceneComponent.SetVisibility` (`/Game/Actors/BP_EnlargedPatient.StaticMesh` (`self.BPEnlargedPatientRef`)) false false)
  (`PrimitiveComponent.SetCollisionEnabled` (`/Game/Actors/BP_EnlargedPatient.StaticMesh` (`self.BPEnlargedPatientRef`)) "NoCollision")
  (`SceneComponent.SetVisibility` (`/Game/Actors/BP_Patient.PassengerMesh` (`/Game/VRTemplate/Blueprints/VRPawn.BPPatientRef` (`self.VRPawnRef`))) true true)
  (`PrimitiveComponent.SetCollisionEnabled` (`/Game/Actors/BP_Patient.PassengerMesh` (`/Game/VRTemplate/Blueprints/VRPawn.BPPatientRef` (`self.VRPawnRef`))) "QueryAndPhysics")
  (`AudioComponent.Stop` (`self.PulseProcedureAudioComp`))
  ;[1 0 0] is there an bAEDProcdureActive in Pawn?
  (set `self.bProcedureActive` false)
  (`/Game/Utility/BP_ConversationComponent.CompletePendingAction` (`/Game/Actors/BP_Patient.BP_ConversationComponent` (`/Game/VRTemplate/Blueprints/VRPawn.BPPatientRef` (`self.VRPawnRef`)))))

(fn `HandleTargetSelected`
  (params (SelectedTargetID :type "/Game/EnumsStructs/ECarotidTargetID Enum" :default "NewEnumerator0"))
  (if (`self.bProcedureActive`)
    (if (`self.bCorrectTargetFound`)
      _
      (elif (`|EnumEquality` SelectedTargetID (`self.CorrectTargetID`))
        (set `self.bCorrectTargetFound` true)
        (set `self.CurrentFeedbackText` (`self.CorrectFeedbackText`))
        (`AudioComponent.SetSound` (`self.PulseProcedureAudioComp`) "/Game/Assets/Audio/SFX/heartbeatloop.heartbeatloop")
        (`AudioComponent.Play` (`self.PulseProcedureAudioComp`) 0.0)
        (`self.SetAllTargetInteractionEnabled` false)
        ; may not need, goes into a conversation right after procedure
        (`/Game/VRTemplate/Blueprints/VRPawn.SetMenuInteractionEnabled` (`self.VRPawnRef`) true)
        (`/Game/VRTemplate/Blueprints/VRPawn.ShowConversationInstruction` (`self.VRPawnRef`) "Click OK to continue." false false (`self.CorrectFeedbackText`))
        (else
          (set `self.CurrentFeedbackText` (`self.IncorrectFeedbackText`))
          (`/Game/VRTemplate/Blueprints/VRPawn.ShowConversationInstruction` (`self.VRPawnRef`) (`self.DefaultInstructionText`) true false (`self.IncorrectFeedbackText`))
          ;[1 0 0] have to handle spam (maybe associate with clicking the button instead)
          (`AudioComponent.SetSound` (`self.PulseProcedureAudioComp`) "/Game/Assets/Audio/SFX/booing.booing")
          (`AudioComponent.Play` (`self.PulseProcedureAudioComp`) 0.0))))))

(fn `InitializeTargetWidgets`
  (bind _aswbp_carotid_target (cast `/Game/Widgets/WBP_CarotidTarget` (`WidgetComponent.GetUserWidgetObject` (`self.CarotidTarget_Left`))))
  (set `self.CarotidTargetWidgetRef` _aswbp_carotid_target)
  (set `/Game/Widgets/WBP_CarotidTarget.ProcedureReference` self _aswbp_carotid_target)
  (set `/Game/Widgets/WBP_CarotidTarget.TargetID` "NewEnumerator0" _aswbp_carotid_target)
  (bind _aswbp_carotid_target_2 (cast `/Game/Widgets/WBP_CarotidTarget` (`WidgetComponent.GetUserWidgetObject` (`self.WrongTarget_Head`))))
  (set `self.HeadTargetWidgetRef` _aswbp_carotid_target_2)
  (set `/Game/Widgets/WBP_CarotidTarget.ProcedureReference` self _aswbp_carotid_target_2)
  (set `/Game/Widgets/WBP_CarotidTarget.TargetID` "NewEnumerator1" _aswbp_carotid_target_2)
  (bind _aswbp_carotid_target_3 (cast `/Game/Widgets/WBP_CarotidTarget` (`WidgetComponent.GetUserWidgetObject` (`self.WrongTarget_Chest`))))
  (set `self.ChestTargetWidgetRef` _aswbp_carotid_target_3)
  (set `/Game/Widgets/WBP_CarotidTarget.ProcedureReference` self _aswbp_carotid_target_3)
  (set `/Game/Widgets/WBP_CarotidTarget.TargetID` "NewEnumerator2" _aswbp_carotid_target_3)
  (bind _aswbp_carotid_target_4 (cast `/Game/Widgets/WBP_CarotidTarget` (`WidgetComponent.GetUserWidgetObject` (`self.WrongTarget_Arm`))))
  (set `self.ArmTargetWidgetRef` _aswbp_carotid_target_4)
  (set `/Game/Widgets/WBP_CarotidTarget.ProcedureReference` self _aswbp_carotid_target_4)
  (set `/Game/Widgets/WBP_CarotidTarget.TargetID` "NewEnumerator3" _aswbp_carotid_target_4)
  (bind _aswbp_carotid_target_5 (cast `/Game/Widgets/WBP_CarotidTarget` (`WidgetComponent.GetUserWidgetObject` (`self.WrongTarget_Abdomen`))))
  (set `self.AbdomenTargetWidgetRef` _aswbp_carotid_target_5)
  (set `/Game/Widgets/WBP_CarotidTarget.ProcedureReference` self _aswbp_carotid_target_5)
  (set `/Game/Widgets/WBP_CarotidTarget.TargetID` "NewEnumerator4" _aswbp_carotid_target_5))

(fn `RestoreProcedureDisplay`
  (if (`self.bCorrectTargetFound`)
    (`self.SetAllTargetInteractionEnabled` false)
    (`/Game/VRTemplate/Blueprints/VRPawn.ShowConversationInstruction` (`self.VRPawnRef`) (`self.CompleteInstructionText`) false false (`self.CorrectFeedbackText`))
    (else
      (`self.SetAllTargetInteractionEnabled` true)
      (`/Game/VRTemplate/Blueprints/VRPawn.ShowConversationInstruction` (`self.VRPawnRef`) (`self.DefaultInstructionText`) true true (`self.CurrentFeedbackText`)))))

(fn `SetAllTargetInteractionEnabled`
  (params (Enabled :type Boolean))
  (if Enabled
    (bind _aswbp_carotid_target (cast `/Game/Widgets/WBP_CarotidTarget` (`WidgetComponent.GetUserWidgetObject` (`self.CarotidTarget_Left`))))
    (`Widget.SetIsEnabled` (`/Game/Widgets/WBP_CarotidTarget.PulseTargetButton` _aswbp_carotid_target) true)
    (bind _aswbp_carotid_target_2 (cast `/Game/Widgets/WBP_CarotidTarget` (`WidgetComponent.GetUserWidgetObject` (`self.WrongTarget_Head`))))
    (`Widget.SetIsEnabled` (`/Game/Widgets/WBP_CarotidTarget.PulseTargetButton` _aswbp_carotid_target_2) true)
    (bind _aswbp_carotid_target_3 (cast `/Game/Widgets/WBP_CarotidTarget` (`WidgetComponent.GetUserWidgetObject` (`self.WrongTarget_Arm`))))
    (`Widget.SetIsEnabled` (`/Game/Widgets/WBP_CarotidTarget.PulseTargetButton` _aswbp_carotid_target_3) true)
    (bind _aswbp_carotid_target_4 (cast `/Game/Widgets/WBP_CarotidTarget` (`WidgetComponent.GetUserWidgetObject` (`self.WrongTarget_Abdomen`))))
    (`Widget.SetIsEnabled` (`/Game/Widgets/WBP_CarotidTarget.PulseTargetButton` _aswbp_carotid_target_4) true)
    (bind _aswbp_carotid_target_5 (cast `/Game/Widgets/WBP_CarotidTarget` (`WidgetComponent.GetUserWidgetObject` (`self.WrongTarget_Chest`))))
    (`Widget.SetIsEnabled` (`/Game/Widgets/WBP_CarotidTarget.PulseTargetButton` _aswbp_carotid_target_5) true)
    (else
      (bind _aswbp_carotid_target_6 (cast `/Game/Widgets/WBP_CarotidTarget` (`WidgetComponent.GetUserWidgetObject` (`self.CarotidTarget_Left`))))
      (`Widget.SetIsEnabled` (`/Game/Widgets/WBP_CarotidTarget.PulseTargetButton` _aswbp_carotid_target_6) false)
      (bind _aswbp_carotid_target_7 (cast `/Game/Widgets/WBP_CarotidTarget` (`WidgetComponent.GetUserWidgetObject` (`self.WrongTarget_Head`))))
      (`Widget.SetIsEnabled` (`/Game/Widgets/WBP_CarotidTarget.PulseTargetButton` _aswbp_carotid_target_7) false)
      (bind _aswbp_carotid_target_8 (cast `/Game/Widgets/WBP_CarotidTarget` (`WidgetComponent.GetUserWidgetObject` (`self.WrongTarget_Arm`))))
      (`Widget.SetIsEnabled` (`/Game/Widgets/WBP_CarotidTarget.PulseTargetButton` _aswbp_carotid_target_8) false)
      (bind _aswbp_carotid_target_9 (cast `/Game/Widgets/WBP_CarotidTarget` (`WidgetComponent.GetUserWidgetObject` (`self.WrongTarget_Abdomen`))))
      (`Widget.SetIsEnabled` (`/Game/Widgets/WBP_CarotidTarget.PulseTargetButton` _aswbp_carotid_target_9) false)
      (bind _aswbp_carotid_target_10 (cast `/Game/Widgets/WBP_CarotidTarget` (`WidgetComponent.GetUserWidgetObject` (`self.WrongTarget_Chest`))))
      (`Widget.SetIsEnabled` (`/Game/Widgets/WBP_CarotidTarget.PulseTargetButton` _aswbp_carotid_target_10) false))))

(fn `SetUpPulseCheck`
  (params (RequestingConversationComponent :type "/Game/Utility/BP_ConversationComponent Object Reference"))
  ; Still want to force anything out of their hands
  (`/Game/VRTemplate/Blueprints/VRPawn.ForceReleaseObject` (`self.VRPawnRef`)))

(fn `ShowHideAllTargets`
  (params (Hide :type Boolean))
  (if Hide
    (`SceneComponent.SetVisibility` (`self.CarotidTarget_Left`) false false)
    (`SceneComponent.SetVisibility` (`self.WrongTarget_Head`) false true)
    (`SceneComponent.SetVisibility` (`self.WrongTarget_Arm`) false true)
    (`SceneComponent.SetVisibility` (`self.WrongTarget_Abdomen`) false true)
    (`SceneComponent.SetVisibility` (`self.WrongTarget_Chest`) false true)
    (else
      (`SceneComponent.SetVisibility` (`self.CarotidTarget_Left`) true false)
      (`SceneComponent.SetVisibility` (`self.WrongTarget_Head`) true true)
      (`SceneComponent.SetVisibility` (`self.WrongTarget_Arm`) true true)
      (`SceneComponent.SetVisibility` (`self.WrongTarget_Abdomen`) true true)
      (`SceneComponent.SetVisibility` (`self.WrongTarget_Chest`) true true))))

(fn `StartProcedure`
  (params (RequestingConversationComponent :type "/Game/Utility/BP_ConversationComponent Object Reference"))
  (bind _output_get (set `self.RequestingConversationComponent` RequestingConversationComponent))
  ; only forces drop, no props to set
  (`self.SetUpPulseCheck` _output_get)
  (set `self.bProcedureActive` true)
  (set `self.bCorrectTargetFound` false)
  (set `self.CurrentFeedbackText` "")
  (`/Engine/EditorBlueprintResources/StandardMacros.IsValid` (`self.VRPawnRef`)
    (:`Is Valid`
      _)
    (:`Is Not Valid`
      (bind _asvrpawn (cast `/Game/VRTemplate/Blueprints/VRPawn` (`GameplayStatics.GetPlayerPawn` 0)))
      (set `self.VRPawnRef` _asvrpawn)))
  (`/Game/VRTemplate/Blueprints/VRPawn.ShowConversationInstruction` (`self.VRPawnRef`) (`self.DefaultInstructionText`) true true "")
  (`SceneComponent.SetVisibility` (`/Game/Actors/BP_Patient.PassengerMesh` (`/Game/VRTemplate/Blueprints/VRPawn.BPPatientRef` (`self.VRPawnRef`))) false true)
  (`PrimitiveComponent.SetCollisionEnabled` (`/Game/Actors/BP_Patient.PassengerMesh` (`/Game/VRTemplate/Blueprints/VRPawn.BPPatientRef` (`self.VRPawnRef`))) "NoCollision")
  (`/Game/Actors/BP_EnlargedPatient.ShowEnlargedPatient` (`self.BPEnlargedPatientRef`))
  (`/Game/VRTemplate/Blueprints/VRPawn.SetMenuInteractionEnabled` (`self.VRPawnRef`) true)
  (`self.ShowHideAllTargets` false))

(fn `UserConstructionScript`)