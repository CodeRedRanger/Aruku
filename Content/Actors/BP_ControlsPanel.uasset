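; BP_ControlsPanel is an actor that hosts the WBP_ControlsWReturn controls screen on a widget component.
; On BeginPlay it hides the widget, disables its collision and binds an event to the widget's return click.
; HandleReturnButtonClicked hides the widget and disables collision again; nothing here shows the panel.
; Unconnected nodes for hiding the root and setting the VRPawn menu state never run.
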(event `self.ReceiveBeginPlay`
  (`SceneComponent.SetVisibility` (`self.Widget`) false false)
  (`SceneComponent.SetHiddenInGame` (`self.Widget`) true false)
  (`PrimitiveComponent.SetCollisionEnabled` (`self.Widget`) "NoCollision")
  (bind _aswbp_controls_wreturn (cast `/Game/Widgets/WBP_ControlsWReturn` (`WidgetComponent.GetUserWidgetObject` (`self.Widget`))))
  (bind _output_get (set `self.WBP ControlsWReturn` _aswbp_controls_wreturn))
  (add `/Game/Widgets/WBP_ControlsWReturn.OnReturnClicked` _output_get (`|CreateDelegate` :!event `HandleReturnButtonClicked`)))

(fn `HandleReturnButtonClicked`
  (`SceneComponent.SetVisibility` (`self.Widget`) false false)
  (`PrimitiveComponent.SetCollisionEnabled` (`self.Widget`) "NoCollision"))

(fn `UserConstructionScript`)