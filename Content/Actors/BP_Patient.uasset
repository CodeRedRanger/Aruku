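; Patient NPC for a VR emergency-care interaction, handling conversation and procedures such as carotid pulse and AED use.
; On BeginPlay it registers with the VR pawn, caches its outcome meter widget and disables passenger mesh collision.
; InteractionRange overlaps notify the conversation component of player and AED presence, using an overlap count to debounce the player.
; Player entry restores an active procedure display or shows the talk prompt, while exit hides prompts and menus.
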(event `self.ReceiveBeginPlay`
  ; Needed for other NPCs to set the conversation node of patient
  (bind _asvrpawn (cast `/Game/VRTemplate/Blueprints/VRPawn` (`GameplayStatics.GetPlayerPawn` 0)))
  (bind _output_get (set `self.VRPawn` _asvrpawn))
  (set `/Game/VRTemplate/Blueprints/VRPawn.BPPatientRef` self _output_get)
  (bind _aswbp_outcome_meter (cast `/Game/Widgets/WBP_OutcomeMeter` (`WidgetComponent.GetUserWidgetObject` (`self.OutcomeMeterWidget`))))
  (set `self.OutcomeMeterRef` _aswbp_outcome_meter)
  (`PrimitiveComponent.SetCollisionEnabled` (`self.PassengerMesh`) "NoCollision"))

(event `self.InteractionRange.OnComponentBeginOverlap`
  (params (OverlappedComponent :type "PrimitiveComponent Object Reference") (OtherActor :type "Actor Object Reference") (OtherComp :type "PrimitiveComponent Object Reference") (OtherBodyIndex :type Integer) (bFromSweep :type Boolean) (SweepResult :type "HitResult Structure (by ref)"))
  (bind _asvrpawn (cast `/Game/VRTemplate/Blueprints/VRPawn` OtherActor)
    (:`then`
      (set `self.VRPawn` _asvrpawn)
      (set `/Game/VRTemplate/Blueprints/VRPawn.ActiveConversationComponent` (`self.BP_ConversationComponent`) (`self.VRPawn`))
      (set `self.PlayerOverlapCount` (+ (`self.PlayerOverlapCount`) 1))
      (if (== (`self.PlayerOverlapCount`) 1)
        (`/Game/Utility/BP_ConversationComponent.HandlePlayerEnteredPatientArea` (`self.BP_ConversationComponent`))
        (set `/Game/VRTemplate/Blueprints/VRPawn.NPCName` (`self.NPCName`) (`self.VRPawn`))
        (set `/Game/VRTemplate/Blueprints/VRPawn.BPPatientRef` self (`self.VRPawn`))
        (if (`|EnumEquality` (`/Game/VRTemplate/Blueprints/VRPawn.ActiveMenuState` (`self.VRPawn`)) "NewEnumerator0")
          (if (`/Game/Utility/BP_ConversationComponent.bWaitingForAction` (`self.BP_ConversationComponent`))
            (if (`/Game/Actors/BP_CarotidPulseProcedure.bProcedureActive` (`/Game/Utility/BP_ConversationComponent.CarotidPulseProcedureRef` (`self.BP_ConversationComponent`)))
              (`/Game/Actors/BP_CarotidPulseProcedure.RestoreProcedureDisplay` (`/Game/Utility/BP_ConversationComponent.CarotidPulseProcedureRef` (`self.BP_ConversationComponent`)))
              (elif (`/Game/Actors/BP_AEDProcedure.bProcedureActive` (`/Game/Utility/BP_ConversationComponent.AEDProcedureRef` (`self.BP_ConversationComponent`)))
                (`/Game/Actors/BP_AEDProcedure.RestoreProcedureDisplay` (`/Game/Utility/BP_ConversationComponent.AEDProcedureRef` (`self.BP_ConversationComponent`)))))
            (else
              (`/Game/VRTemplate/Blueprints/VRPawn.ShowTalkPrompt` (`self.VRPawn`)))))))
    (:`CastFailed`
      (bind _asbp_aed (cast `/Game/Actors/BP_AED` OtherActor))
      (set `/Game/Utility/BP_ConversationComponent.bAEDInPatientArea` true (`self.BP_ConversationComponent`))
      (set `self.BPAEDRef` _asbp_aed)
      (`/Game/Utility/BP_ConversationComponent.HandleAEDEnteredPatientArea` (`self.BP_ConversationComponent`)))))

(event `self.InteractionRange.OnComponentEndOverlap`
  (params (OverlappedComponent :type "PrimitiveComponent Object Reference") (OtherActor :type "Actor Object Reference") (OtherComp :type "PrimitiveComponent Object Reference") (OtherBodyIndex :type Integer))
  (bind _asvrpawn (cast `/Game/VRTemplate/Blueprints/VRPawn` OtherActor)
    (:`then`
      (set `self.PlayerOverlapCount` (`KismetMathLibrary.Max` (- (`self.PlayerOverlapCount`) 1)))
      (if (== (`self.PlayerOverlapCount`) 0)
        (`/Game/Utility/BP_ConversationComponent.HandlePlayerLeftPatientArea` (`self.BP_ConversationComponent`))
        (`/Game/VRTemplate/Blueprints/VRPawn.HideTalkPrompt` _asvrpawn)
        (`/Game/VRTemplate/Blueprints/VRPawn.CloseConversationMenu` _asvrpawn)
        (`/Game/VRTemplate/Blueprints/VRPawn.HideBindInstructionWidget` (`self.VRPawn`))))
    (:`CastFailed`
      (cast `/Game/Actors/BP_AED` OtherActor)
      (set `/Game/Utility/BP_ConversationComponent.bAEDInPatientArea` false (`self.BP_ConversationComponent`)))))

(fn `UserConstructionScript`)