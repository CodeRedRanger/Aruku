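; BP_Boat is a grabbable boat that gives the VR player a timed ride along a spline.
; Grabbing it in a specific game-instance network state flags the VRPawn as riding, stores its offset and starts a timeline scaled by RideDuration.
; The timeline moves and rotates the boat along BoatRideSpline, carrying the pawn by position only.
; On finish, it clears the riding flag and triggers the pawn's right-hand release.
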(event `self.ReceiveTick`
  (params (DeltaSeconds :type "Float (single-precision)"))
  (if (`self.IsPlayerAttached`)
    (`self.K2_SetActorLocation` (`GameplayStatics.GetPlayerPawn` 0) (+ (`self.PlayerRelativeLocation`) (`self.K2_GetActorLocation` self)) false false)
    (`self.K2_SetActorLocation` self (+ (`self.K2_GetActorLocation` self) (0.0 1.0 0.0)) false false)))

(event `self.GrabComponent.OnGrabbed`
  (bind _returnvalue (`GameplayStatics.GetPlayerPawn` 0))
  (bind _asbp_med_game_instance (cast `/Game/Utility/BP_MedGameInstance` (`GameplayStatics.GetGameInstance`)))
  (if (`|EnumEquality` (`/Game/Utility/BP_MedGameInstance.NetworkState` _asbp_med_game_instance) "NewEnumerator0")
    (bind _asvrpawn (cast `/Game/VRTemplate/Blueprints/VRPawn` _returnvalue))
    (set `/Game/VRTemplate/Blueprints/VRPawn.IsOnBoatRide` true _asvrpawn)
    (set `self.PlayerRelativeLocation` (- (`self.K2_GetActorLocation` _returnvalue) (`self.K2_GetActorLocation` self)))
    (set `self.PlayerRelativeRotation` (`self.GetRelativeRotation` (`self.K2_GetActorRotation` (`GameplayStatics.GetPlayerPawn` 0)) (`self.K2_GetActorRotation` self)))
    (`self.MoveOnSpline`)))

(event `End Boat Ride`
  ; WILL BREAK WITHOUT VR PAWN HAVING THE EVENT
  (bind _asvrpawn (cast `/Game/VRTemplate/Blueprints/VRPawn` (`GameplayStatics.GetPlayerPawn` 0)))
  (set `/Game/VRTemplate/Blueprints/VRPawn.IsOnBoatRide` false _asvrpawn)
  (`/Game/VRTemplate/Blueprints/VRPawn.RightReleaseTriggered` _asvrpawn)
  (set `self.IsPlayerAttached` false))

(event `MoveOnSpline`
  (bind _boatridespline (`self.BoatRideSpline`))
  (`/Engine/EditorBlueprintResources/StandardMacros.IsValid` _boatridespline
    (:`Is Valid`
      (`TimelineComponent.SetPlayRate` (`self.BoatRide`) (/ 1.0 (`self.RideDuration`)))
      (bind (_direction _boatridetime) (`Timeline|BoatRide` :!via `PlayFromStart`)
        (:`Update`
          (`self.K2_SetActorLocation` (.location (`SplineComponent.GetTransformAtTime` (`/Game/Actors/BoatRide/BP_BoatRideSpline.BoatRideSplinePath` _boatridespline) _boatridetime "World" false false)))
          (`self.K2_SetActorRotation` (.rotation (`SplineComponent.GetTransformAtTime` (`/Game/Actors/BoatRide/BP_BoatRideSpline.BoatRideSplinePath` _boatridespline) _boatridetime "World" false false)))
          (`self.K2_SetActorLocation` (`GameplayStatics.GetPlayerPawn` 0) (+ (`self.PlayerRelativeLocation`) (`self.K2_GetActorLocation` self)) false false))
        (:`Finished`
          (`self.End Boat Ride`))))))

(fn `AddRotation`
  (params (OtherRotation :type "Rotator Structure") (SelfRotation :type "Rotator Structure"))
  (returns (NewRotation :type "Rotator Structure"))
  (return (`KismetMathLibrary.MakeRotator` (+ (.roll OtherRotation) (.roll SelfRotation)) (+ (.pitch OtherRotation) (.pitch SelfRotation)) (+ (.yaw OtherRotation) (.yaw SelfRotation)))))

(fn `GetRelativeRotation`
  (params (OtherRotation :type "Rotator Structure") (SelfRotation :type "Rotator Structure"))
  (returns (RelativeRotation :type "Rotator Structure"))
  (bind (_x _y _z) (`KismetMathLibrary.BreakRotIntoAxes` OtherRotation))
  (bind (_x_2 _y_2 _z_2) (`KismetMathLibrary.BreakRotIntoAxes` SelfRotation))
  (return (`KismetMathLibrary.MakeRotationFromAxes` (- _x _x_2) (- _y _y_2) (- _z _z_2))))

(fn `UserConstructionScript`)