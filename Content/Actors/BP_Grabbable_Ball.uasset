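; BP_Grabbable_Ball is a VR ball that can be grabbed and thrown with its held state networked.
; GrabComponent events ask the VRPawn for a network grab with hand and relative offset, or a release with controller velocities.
; Non-authority instances disable mesh physics after requesting release.
; While held by a non-locally controlled pawn, Tick teleports the ball to that pawn's networked hand transform plus the grab offset, forcing a fixed scale.
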(event `self.ReceiveTick`
  (params (DeltaSeconds :type "Float (single-precision)"))
  (bind _returnvalue (`self.GetHoldingPawn`))
  (bind (_returnvalue_location _returnvalue_rotation) (`KismetMathLibrary.BreakTransform` (`KismetMathLibrary.ComposeTransforms` (`self.GetGrabRelativeTransform`) (`VRPawnCustom.GetNetworkGrabHandTransform` _returnvalue (`self.GetHoldingHand`)))))
  (if (`self.IsNetworkHeld`)
    (`/Engine/EditorBlueprintResources/StandardMacros.IsValid` _returnvalue
      (:`Is Valid`
        (if (not (`Pawn.IsLocallyControlled` _returnvalue))
          (`self.K2_SetActorTransform` (`KismetMathLibrary.MakeTransform` _returnvalue_location _returnvalue_rotation (0.05 0.05 0.05)) false true))))))

(event `self.GrabComponent.OnGrabbed`
  (bind _motioncontrollerref (`/Game/VRTemplate/Blueprints/GrabComponent.MotionControllerRef` (`self.GrabComponent`)))
  (bind (_returnvalue_location _returnvalue_rotation) (`KismetMathLibrary.BreakTransform` (`KismetMathLibrary.MakeRelativeTransform` (`self.GetTransform`) (`SceneComponent.K2_GetComponentToWorld` (`/Game/VRTemplate/Blueprints/GrabComponent.MotionControllerRef` (`self.GrabComponent`))))))
  (bind _asvrpawn (cast `/Game/VRTemplate/Blueprints/VRPawn` (`ActorComponent.GetOwner` _motioncontrollerref)))
  (if (== _motioncontrollerref (`/Game/VRTemplate/Blueprints/VRPawn.MotionControllerLeftGrip` _asvrpawn))
    (set `self.CurrentGrabHand` "Left")
    (else
      (bind _output_get (set `self.CurrentGrabHand` "Right"))))
  (`VRPawnCustom.RequestNetworkGrab` _asvrpawn self _output_get (`KismetMathLibrary.MakeTransform` _returnvalue_location _returnvalue_rotation)))

(event `self.GrabComponent.OnDropped`
  (bind _motioncontrollerref (`/Game/VRTemplate/Blueprints/GrabComponent.MotionControllerRef` (`self.GrabComponent`)))
  (bind _outangularvelocity (`MotionControllerComponent.GetAngularVelocity` _motioncontrollerref))
  (`/Engine/EditorBlueprintResources/StandardMacros.IsValid` _motioncontrollerref
    (:`Is Valid`
      (bind _asvrpawn (cast `/Game/VRTemplate/Blueprints/VRPawn` (`ActorComponent.GetOwner` _motioncontrollerref)))
      (`VRPawnCustom.RequestNetworkRelease` _asvrpawn self (`MotionControllerComponent.GetLinearVelocity` _motioncontrollerref) (`KismetMathLibrary.MakeVector` (.roll _outangularvelocity) (.pitch _outangularvelocity) (.yaw _outangularvelocity)))
      (`/Engine/EditorBlueprintResources/ActorMacros.Switch Has Authority`
        (:`Remote`
          (`PrimitiveComponent.SetSimulatePhysics` (`self.StaticMesh`) false))))
    (:`Is Not Valid`
      (`KismetSystemLibrary.PrintString` "Motion Controller no longer valid" true true (struct :`G` 0.66 :`B` 1.0 :`A` 1.0) 20.0))))

(fn `UserConstructionScript`)