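; BP_AEDProcedure runs the VR AED procedure on a patient, from pad placement to a no-shock result.
; Starting it positions the AED and swaps the patient for an enlarged stand-in; pads snap to front and back points or reset when leaving the boundary.
; With both pads placed, heartbeat effects start and power unlocks a timed no-shock message.
; EndProcedure hides the equipment and, if the heart effect exists, restores the patient and completes the pending conversation action.
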(event `self.ReceiveBeginPlay`
  (`SceneComponent.SetVisibility` (`/Game/Actors/BP_EnlargedPatient.StaticMesh` (`self.BPEnlargedPatientRef`)) false false)
  (bind _asvrpawn (cast `/Game/VRTemplate/Blueprints/VRPawn` (`GameplayStatics.GetPlayerPawn` 0)))
  (set `self.VRPawnRef` _asvrpawn)
  (set `/Game/Actors/BP_EnlargedPatient.AEDProcedureRef` self (`self.BPEnlargedPatientRef`))
  (`PrimitiveComponent.SetCollisionEnabled` (`/Game/Actors/BP_EnlargedPatient.StaticMesh` (`self.BPEnlargedPatientRef`)) "NoCollision"))

(event `self.AEDPadBoundary.OnComponentEndOverlap`
  (params (OverlappedComponent :type "PrimitiveComponent Object Reference") (OtherActor :type "Actor Object Reference") (OtherComp :type "PrimitiveComponent Object Reference") (OtherBodyIndex :type Integer))
  (bind _asbp_aedpad (cast `/Game/Actors/BP_AEDPad` OtherActor))
  (set `self.CurrentAEDPad` _asbp_aedpad)
  (`/Game/Actors/BP_AEDPad.ResetPad` (`self.CurrentAEDPad`)))

(event `AEDTimerEvent`
  (`/Game/VRTemplate/Blueprints/VRPawn.ShowConversationInstruction` (`self.VRPawnRef`) (`self.AEDNoShock`) true true "")
  ; skip shock anyway
  (set `self.CurrentProcedureState` "NewEnumerator4")
  (set `self.CurrentProcedureState` "NewEnumerator5")
  (`/Game/VRTemplate/Blueprints/VRPawn.ShowOKOnly` (`self.VRPawnRef`)))

(fn `CompleteBackPadPlacement`
  (params (PadReference :type "/Game/Actors/BP_AEDPad Object Reference"))
  (locals (CurrentPad :type "/Game/Actors/BP_AEDPad Object Reference"))
  (bind _output_get (set `local.CurrentPad` PadReference))
  (set `/Game/Actors/BP_AEDPad.bCorrectlyPlaced` true _output_get)
  (`/Game/VRTemplate/Blueprints/VRPawn.ForceReleaseObject` (`self.VRPawnRef`))
  (set `/Game/VRTemplate/Blueprints/GrabComponent.GrabType` "NewEnumerator0" (`/Game/Actors/BP_AEDPad.GrabComponent` (`local.CurrentPad`)))
  (`PrimitiveComponent.SetSimulatePhysics` (`/Game/Actors/BP_AEDPad.StaticMesh` (`local.CurrentPad`)) false)
  (set `self.bBackPadPlaced` true)
  (`self.K2_AttachToComponent` (`local.CurrentPad`) (`/Game/Actors/BP_EnlargedPatient.BackPadSnapPoint` (`self.BPEnlargedPatientRef`)) "None" "SnapToTarget" "SnapToTarget" "KeepWorld" true)
  (if (and (`self.bFrontPadPlaced`) (`self.bBackPadPlaced`))
    (bind _returnvalue (`GameplayStatics.SpawnEmitterAtLocation` "/Game/END_Starter/VFX/PulsingHeart/P_Heart_Pulsing.P_Heart_Pulsing" (`SceneComponent.K2_GetComponentLocation` (`/Game/Actors/BP_EnlargedPatient.BackPadSnapPoint` (`self.BPEnlargedPatientRef`))) (struct) (0.5 0.1 0.3)))
    (set `self.HeartParticleRef` _returnvalue)
    (`AudioComponent.SetSound` (`self.AEDProcedureAudioComp`) "/Game/Assets/Audio/SFX/heartbeatloop.heartbeatloop")
    (`AudioComponent.Play` (`self.AEDProcedureAudioComp`) 0.0)
    (`/Game/VRTemplate/Blueprints/VRPawn.ShowConversationInstruction` (`self.VRPawnRef`) (`self.AEDUseInstructionText`) true true "")
    (set `self.CurrentProcedureState` "NewEnumerator2")
    (`PrimitiveComponent.SetCollisionEnabled` (`/Game/Actors/BP_EnlargedPatient.StaticMesh` (`self.BPEnlargedPatientRef`)) "NoCollision")))

(fn `CompleteFrontPadPlacement`
  (params (PadReference :type "/Game/Actors/BP_AEDPad Object Reference"))
  (locals (CurrentPad :type "/Game/Actors/BP_AEDPad Object Reference"))
  (bind _output_get (set `local.CurrentPad` PadReference))
  (set `/Game/Actors/BP_AEDPad.bCorrectlyPlaced` true _output_get)
  (`/Game/VRTemplate/Blueprints/VRPawn.ForceReleaseObject` (`self.VRPawnRef`))
  (set `/Game/VRTemplate/Blueprints/GrabComponent.GrabType` "NewEnumerator0" (`/Game/Actors/BP_AEDPad.GrabComponent` (`local.CurrentPad`)))
  (`PrimitiveComponent.SetSimulatePhysics` (`/Game/Actors/BP_AEDPad.StaticMesh` (`local.CurrentPad`)) false)
  (set `self.bFrontPadPlaced` true)
  (`self.K2_AttachToComponent` (`local.CurrentPad`) (`/Game/Actors/BP_EnlargedPatient.FrontPadSnapPoint` (`self.BPEnlargedPatientRef`)) "None" "SnapToTarget" "SnapToTarget" "KeepWorld" true)
  (if (and (`self.bFrontPadPlaced`) (`self.bBackPadPlaced`))
    (bind _returnvalue (`GameplayStatics.SpawnEmitterAtLocation` "/Game/END_Starter/VFX/PulsingHeart/P_Heart_Pulsing.P_Heart_Pulsing" (`SceneComponent.K2_GetComponentLocation` (`/Game/Actors/BP_EnlargedPatient.BackPadSnapPoint` (`self.BPEnlargedPatientRef`))) (struct) (0.5 0.1 0.3)))
    (set `self.HeartParticleRef` _returnvalue)
    (`AudioComponent.SetSound` (`self.AEDProcedureAudioComp`) "/Game/Assets/Audio/SFX/heartbeatloop.heartbeatloop")
    (`AudioComponent.Play` (`self.AEDProcedureAudioComp`) 0.0)
    (`/Game/VRTemplate/Blueprints/VRPawn.ShowConversationInstruction` (`self.VRPawnRef`) (`self.AEDUseInstructionText`) true true "")
    (set `self.CurrentProcedureState` "NewEnumerator2")
    (`PrimitiveComponent.SetCollisionEnabled` (`/Game/Actors/BP_EnlargedPatient.StaticMesh` (`self.BPEnlargedPatientRef`)) "NoCollision")))

(fn `EndProcedure`
  (bind _heartparticleref (`self.HeartParticleRef`))
  (`SceneComponent.SetVisibility` (`/Game/Actors/BP_AED.StaticMesh` (`self.BPAEDRef`)) false true)
  (`SceneComponent.SetHiddenInGame` (`/Game/Actors/BP_AED.StaticMesh` (`self.BPAEDRef`)) true true)
  (`PrimitiveComponent.SetCollisionEnabled` (`/Game/Actors/BP_AED.StaticMesh` (`self.BPAEDRef`)) "NoCollision")
  (`PrimitiveComponent.SetCollisionEnabled` (`/Game/Actors/BP_AED.AEDButtons` (`self.BPAEDRef`)) "NoCollision")
  (`SceneComponent.SetVisibility` (`/Game/Actors/BP_AEDPad.StaticMesh` (`self.FrontPadRef`)) false true)
  (`self.SetActorHiddenInGame` (`self.FrontPadRef`) true)
  (`PrimitiveComponent.SetCollisionEnabled` (`/Game/Actors/BP_AEDPad.StaticMesh` (`self.FrontPadRef`)) "NoCollision")
  (`SceneComponent.SetVisibility` (`/Game/Actors/BP_AEDPad.StaticMesh` (`self.BackPadRef`)) false true)
  (`self.SetActorHiddenInGame` (`self.BackPadRef`) true)
  (`PrimitiveComponent.SetCollisionEnabled` (`/Game/Actors/BP_AEDPad.StaticMesh` (`self.BackPadRef`)) "NoCollision")
  (`SceneComponent.SetHiddenInGame` (`/Game/Actors/BP_EnlargedPatient.StaticMesh` (`self.BPEnlargedPatientRef`)) true false)
  (`SceneComponent.SetVisibility` (`/Game/Actors/BP_EnlargedPatient.StaticMesh` (`self.BPEnlargedPatientRef`)) false false)
  (`PrimitiveComponent.SetCollisionEnabled` (`/Game/Actors/BP_EnlargedPatient.StaticMesh` (`self.BPEnlargedPatientRef`)) "NoCollision")
  (`SceneComponent.SetVisibility` (`/Game/Actors/BP_Patient.PassengerMesh` (`/Game/VRTemplate/Blueprints/VRPawn.BPPatientRef` (`self.VRPawnRef`))) false true)
  (`/Engine/EditorBlueprintResources/StandardMacros.IsValid` _heartparticleref
    (:`Is Valid`
      (`ActorComponent.K2_DestroyComponent` _heartparticleref)
      (`AudioComponent.Stop` (`self.AEDProcedureAudioComp`))
      (`SceneComponent.SetVisibility` (`/Game/Actors/BP_Patient.PassengerMesh` (`/Game/VRTemplate/Blueprints/VRPawn.BPPatientRef` (`self.VRPawnRef`))) true true)
      (set `self.bProcedureActive` false)
      (`/Game/Utility/BP_ConversationComponent.CompletePendingAction` (`/Game/Actors/BP_Patient.BP_ConversationComponent` (`/Game/VRTemplate/Blueprints/VRPawn.BPPatientRef` (`self.VRPawnRef`)))))))

(fn `HandlePowerButtonClicked`
  ; Could branch and check that ProcedureActive is true, but doesn't matter since AED disappears at end of procedure
  (if (`|EnumEquality` (`self.CurrentProcedureState`) "NewEnumerator2")
    (set `self.CurrentProcedureState` "NewEnumerator3")
    (set `self.bAEDPoweredOn` true)
    (bind _aswbp_aedbuttons (cast `/Game/Widgets/WBP_AEDButtons` (`WidgetComponent.GetWidget` (`/Game/Actors/BP_AED.AEDButtons` (`self.BPAEDRef`)))))
    (`Widget.SetIsEnabled` (`/Game/Widgets/WBP_AEDButtons.PowerButton` _aswbp_aedbuttons) false)
    (`/Game/VRTemplate/Blueprints/VRPawn.ShowConversationInstruction` (`self.VRPawnRef`) "" true true "")
    (`GameplayStatics.PlaySound2D` "/Engine/EngineSounds/WhiteNoise.WhiteNoise" 1.0 1.0 0.0 null null)
    (`KismetSystemLibrary.K2_SetTimerDelegate` (`|CreateDelegate` :!event `AEDTimerEvent`) 3.0)
    (else
      (`/Game/VRTemplate/Blueprints/VRPawn.ShowConversationInstruction` (`self.VRPawnRef`) (`self.AEDNeedsPads`) true true ""))))

(fn `RestoreProcedureDisplay`
  ; display ok button/no shock indicated
  (if (and (`self.bFrontPadPlaced`) (`self.bBackPadPlaced`) (`self.bAEDPoweredOn`))
    (`/Game/VRTemplate/Blueprints/VRPawn.ShowConversationInstruction` (`self.VRPawnRef`) (`self.AEDNoShock`) true true "")
    (else
      ; Power on the AED
      (if (and (`self.bFrontPadPlaced`) (`self.bBackPadPlaced`))
        (`/Game/VRTemplate/Blueprints/VRPawn.ShowConversationInstruction` (`self.VRPawnRef`) (`self.AEDUseInstructionText`) true true "")
        (else
          ; place the pads
          (`/Game/VRTemplate/Blueprints/VRPawn.ShowConversationInstruction` (`self.VRPawnRef`) (`self.AEDAttachPads`) true true ""))))))

(fn `SetUpAED`
  (params (RequestingConversationComponent :type "/Game/Utility/BP_ConversationComponent Object Reference"))
  (bind _frontpadref (`self.FrontPadRef`))
  (bind _aedfloorpoint (`self.AEDFloorPoint`))
  (bind _backpadref (`self.BackPadRef`))
  ; can get rid of input for this and start procedure (AED)
  (`/Game/VRTemplate/Blueprints/VRPawn.ForceReleaseObject` (`self.VRPawnRef`))
  (set `/Game/VRTemplate/Blueprints/GrabComponent.GrabType` "NewEnumerator0" (`/Game/Actors/BP_AED.GrabComponent` (`self.BPAEDRef`)))
  (`PrimitiveComponent.SetSimulatePhysics` (`/Game/Actors/BP_AED.StaticMesh` (`self.BPAEDRef`)) false)
  (`self.K2_SetActorLocation` (`self.BPAEDRef`) (`SceneComponent.K2_GetComponentLocation` _aedfloorpoint) false true)
  (`self.K2_SetActorRotation` (`self.BPAEDRef`) (`SceneComponent.K2_GetComponentRotation` _aedfloorpoint) false)
  (`SceneComponent.SetVisibility` (`/Game/Actors/BP_AEDPad.StaticMesh` (`self.FrontPadRef`)) true true)
  (set `/Game/Actors/BP_AEDPad.HomeTransform` (`self.GetTransform` _frontpadref) _frontpadref)
  (`SceneComponent.SetVisibility` (`/Game/Actors/BP_AEDPad.StaticMesh` (`self.BackPadRef`)) true true)
  (set `/Game/Actors/BP_AEDPad.HomeTransform` (`self.GetTransform` _backpadref) _backpadref))

(fn `StartProcedure`
  (params (RequestingConversationComponent :type "/Game/Utility/BP_ConversationComponent Object Reference"))
  (bind _output_get (set `self.RequestingConversationComponent` RequestingConversationComponent))
  (`self.SetUpAED` _output_get)
  (set `self.bProcedureActive` true)
  (bind _aswbp_aedbuttons (cast `/Game/Widgets/WBP_AEDButtons` (`WidgetComponent.GetUserWidgetObject` (`/Game/Actors/BP_AED.AEDButtons` (`self.BPAEDRef`)))))
  (add `/Game/Widgets/WBP_AEDButtons.OnPowerClicked` _aswbp_aedbuttons (`|CreateDelegate` :!event `HandlePowerButtonClicked`))
  (`/Game/VRTemplate/Blueprints/VRPawn.ShowConversationInstruction` (`self.VRPawnRef`) (`self.AEDAttachPads`) true true "")
  (`SceneComponent.SetVisibility` (`/Game/Actors/BP_Patient.PassengerMesh` (`/Game/VRTemplate/Blueprints/VRPawn.BPPatientRef` (`self.VRPawnRef`))) false true)
  (`SceneComponent.SetVisibility` (`/Game/Actors/BP_EnlargedPatient.StaticMesh` (`self.BPEnlargedPatientRef`)) true false)
  (`PrimitiveComponent.SetCollisionEnabled` (`/Game/Actors/BP_EnlargedPatient.StaticMesh` (`self.BPEnlargedPatientRef`)) "QueryAndPhysics"))

(fn `UserConstructionScript`)