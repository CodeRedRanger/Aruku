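; BP_PatientSpouse is an NPC actor representing the patient's spouse that the VR player can approach to talk with.
; Its interaction range overlap hands the VRPawn its conversation component, name and a self reference, then shows the talk prompt.
; An overlap counter ensures the prompt shows only on first entry, and the prompt and conversation menu close when the count returns to zero.
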(event `self.ReceiveBeginPlay`)

(event `self.InteractionRangeCode.OnComponentBeginOverlap`
  (params (OverlappedComponent :type "PrimitiveComponent Object Reference") (OtherActor :type "Actor Object Reference") (OtherComp :type "PrimitiveComponent Object Reference") (OtherBodyIndex :type Integer) (bFromSweep :type Boolean) (SweepResult :type "HitResult Structure (by ref)"))
  (bind _asvrpawn (cast `/Game/VRTemplate/Blueprints/VRPawn` OtherActor))
  (set `self.VRPawn` _asvrpawn)
  (set `/Game/VRTemplate/Blueprints/VRPawn.ActiveConversationComponent` (`self.BP_ConversationComponent`) (`self.VRPawn`))
  (set `self.PlayerOverlapCount` (+ (`self.PlayerOverlapCount`) 1))
  (if (== (`self.PlayerOverlapCount`) 1)
    (set `/Game/VRTemplate/Blueprints/VRPawn.NPCName` (`self.NPCName`) (`self.VRPawn`))
    ;[1 0 0] Pawn need spouse ref
    (set `/Game/VRTemplate/Blueprints/VRPawn.BPPatientSpouseRef` self (`self.VRPawn`))
    (`/Game/VRTemplate/Blueprints/VRPawn.ShowTalkPrompt` (`self.VRPawn`))))

(event `self.InteractionRangeCode.OnComponentEndOverlap`
  (params (OverlappedComponent :type "PrimitiveComponent Object Reference") (OtherActor :type "Actor Object Reference") (OtherComp :type "PrimitiveComponent Object Reference") (OtherBodyIndex :type Integer))
  (bind _asvrpawn (cast `/Game/VRTemplate/Blueprints/VRPawn` OtherActor))
  (set `self.PlayerOverlapCount` (`KismetMathLibrary.Max` (- (`self.PlayerOverlapCount`) 1)))
  (if (== (`self.PlayerOverlapCount`) 0)
    (`/Game/VRTemplate/Blueprints/VRPawn.HideTalkPrompt` _asvrpawn)
    (`/Game/VRTemplate/Blueprints/VRPawn.CloseConversationMenu` _asvrpawn)))

(fn `UserConstructionScript`)