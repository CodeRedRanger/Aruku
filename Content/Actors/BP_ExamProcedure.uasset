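; Runs a VR medical exam where the player places vitals tools from a med kit onto an enlarged patient.
; Starting swaps in the enlarged patient and reveals placement spheres; tools leaving the kit boundary reset.
; Completion functions snap each tool and show its reading, exposing the OK button once all four are placed.
; EndProcedure restores the patient and completes the pending conversation action; RestoreProcedureDisplay still checks AED state.
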(event `self.ReceiveBeginPlay`
  (`SceneComponent.SetVisibility` (`/Game/Actors/BP_EnlargedPatient.StaticMesh` (`self.BPEnlargedPatientRef`)) false false)
  (bind _asvrpawn (cast `/Game/VRTemplate/Blueprints/VRPawn` (`GameplayStatics.GetPlayerPawn` 0)))
  (set `self.VRPawnRef` _asvrpawn)
  (set `/Game/Actors/BP_EnlargedPatient.ExamProcedureRef` self (`self.BPEnlargedPatientRef`))
  (`PrimitiveComponent.SetCollisionEnabled` (`/Game/Actors/BP_EnlargedPatient.StaticMesh` (`self.BPEnlargedPatientRef`)) "NoCollision"))

(event `self.MedKitItemBoundary.OnComponentEndOverlap`
  (params (OverlappedComponent :type "PrimitiveComponent Object Reference") (OtherActor :type "Actor Object Reference") (OtherComp :type "PrimitiveComponent Object Reference") (OtherBodyIndex :type Integer))
  (bind _asbp_med_kit_item (cast `/Game/Actors/BP_MedKitItem` OtherActor))
  (set `self.CurrentMedKitItemNonLocal` _asbp_med_kit_item)
  (`/Game/Actors/BP_MedKitItem.ResetItem` (`self.CurrentMedKitItemNonLocal`)))

(fn `CompleteBPCuffPlacement`
  (params (KitItemReference :type "/Game/Actors/BP_MedKitItem Object Reference"))
  (locals (CurrentPad :type "/Game/Actors/BP_AEDPad Object Reference") (CurrentMedKitItem :type "/Game/Actors/BP_MedKitItem Object Reference"))
  (bind _output_get (set `local.CurrentMedKitItem` KitItemReference))
  (set `/Game/Actors/BP_MedKitItem.bCorrectlyPlaced` true _output_get)
  (`/Game/VRTemplate/Blueprints/VRPawn.ForceReleaseObject` (`self.VRPawnRef`))
  (set `/Game/VRTemplate/Blueprints/GrabComponent.GrabType` "NewEnumerator0" (`/Game/Actors/BP_MedKitItem.GrabComponent` (`local.CurrentMedKitItem`)))
  (`PrimitiveComponent.SetSimulatePhysics` (`/Game/Actors/BP_MedKitItem.StaticMesh` (`local.CurrentMedKitItem`)) false)
  (`SceneComponent.SetVisibility` (`MedKitItem.LabelWidgetComponent` (`local.CurrentMedKitItem`)) false true)
  (set `self.bBPCuffPlaced` true)
  (`self.K2_AttachToComponent` (`local.CurrentMedKitItem`) (`/Game/Actors/BP_EnlargedPatient.BPCuffSnapPoint` (`self.BPEnlargedPatientRef`)) "None" "SnapToTarget" "SnapToTarget" "KeepWorld" true)
  (`/Game/VRTemplate/Blueprints/VRPawn.ShowConversationInstruction` (`self.VRPawnRef`) (`self.BPCuffValue`) true true "")
  (if (and (`self.bPulseOxPlaced`) (`self.bThermometerPlaced`) (`self.bBPCuffPlaced`) (`self.bStethoscopeHeartPlaced`))
    (set `self.CurrentProcedureState` "NewEnumerator0")
    (`/Game/VRTemplate/Blueprints/VRPawn.ShowConversationInstruction` (`self.VRPawnRef`) (`self.BPCuffValue`) false true "")
    (`PrimitiveComponent.SetCollisionEnabled` (`/Game/VRTemplate/Blueprints/VRPawn.InstructionWidget` (`self.VRPawnRef`)) "QueryOnly")
    (`PrimitiveComponent.SetCollisionEnabled` (`/Game/Actors/BP_EnlargedPatient.StaticMesh` (`self.BPEnlargedPatientRef`)) "NoCollision")))

(fn `CompleteHeartStethoscopePlacement`
  (params (KitItemReference :type "/Game/Actors/BP_MedKitItem Object Reference"))
  (locals (CurrentPad :type "/Game/Actors/BP_AEDPad Object Reference") (CurrentMedKitItem :type "/Game/Actors/BP_MedKitItem Object Reference"))
  (bind _output_get (set `local.CurrentMedKitItem` KitItemReference))
  (set `/Game/Actors/BP_MedKitItem.bCorrectlyPlaced` true _output_get)
  (`/Game/VRTemplate/Blueprints/VRPawn.ForceReleaseObject` (`self.VRPawnRef`))
  (set `/Game/VRTemplate/Blueprints/GrabComponent.GrabType` "NewEnumerator0" (`/Game/Actors/BP_MedKitItem.GrabComponent` (`local.CurrentMedKitItem`)))
  (`PrimitiveComponent.SetSimulatePhysics` (`/Game/Actors/BP_MedKitItem.StaticMesh` (`local.CurrentMedKitItem`)) false)
  (`SceneComponent.SetVisibility` (`MedKitItem.LabelWidgetComponent` (`local.CurrentMedKitItem`)) false true)
  (set `self.bStethoscopeHeartPlaced` true)
  (`self.K2_AttachToComponent` (`local.CurrentMedKitItem`) (`/Game/Actors/BP_EnlargedPatient.StethoscopeHeartSnapPoint` (`self.BPEnlargedPatientRef`)) "None" "SnapToTarget" "SnapToTarget" "KeepWorld" true)
  (`/Game/VRTemplate/Blueprints/VRPawn.ShowConversationInstruction` (`self.VRPawnRef`) (`self.StethoscopeHeartValue`) true true "")
  (if (and (`self.bPulseOxPlaced`) (`self.bThermometerPlaced`) (`self.bBPCuffPlaced`) (`self.bStethoscopeHeartPlaced`))
    (set `self.CurrentProcedureState` "NewEnumerator0")
    (`/Game/VRTemplate/Blueprints/VRPawn.ShowConversationInstruction` (`self.VRPawnRef`) (`self.StethoscopeHeartValue`) false true "")
    (`PrimitiveComponent.SetCollisionEnabled` (`/Game/VRTemplate/Blueprints/VRPawn.InstructionWidget` (`self.VRPawnRef`)) "QueryOnly")
    (`PrimitiveComponent.SetCollisionEnabled` (`/Game/Actors/BP_EnlargedPatient.StaticMesh` (`self.BPEnlargedPatientRef`)) "NoCollision")))

(fn `CompletePulseOxPlacement`
  (params (KitItemReference :type "/Game/Actors/BP_MedKitItem Object Reference"))
  (locals (CurrentPad :type "/Game/Actors/BP_AEDPad Object Reference") (CurrentMedKitItem :type "/Game/Actors/BP_MedKitItem Object Reference"))
  (bind _output_get (set `local.CurrentMedKitItem` KitItemReference))
  (set `/Game/Actors/BP_MedKitItem.bCorrectlyPlaced` true _output_get)
  (`/Game/VRTemplate/Blueprints/VRPawn.ForceReleaseObject` (`self.VRPawnRef`))
  (set `/Game/VRTemplate/Blueprints/GrabComponent.GrabType` "NewEnumerator0" (`/Game/Actors/BP_MedKitItem.GrabComponent` (`local.CurrentMedKitItem`)))
  (`PrimitiveComponent.SetSimulatePhysics` (`/Game/Actors/BP_MedKitItem.StaticMesh` (`local.CurrentMedKitItem`)) false)
  (`SceneComponent.SetVisibility` (`MedKitItem.LabelWidgetComponent` (`local.CurrentMedKitItem`)) false true)
  (set `self.bPulseOxPlaced` true)
  (`self.K2_AttachToComponent` (`local.CurrentMedKitItem`) (`/Game/Actors/BP_EnlargedPatient.PulseOxSnapPoint` (`self.BPEnlargedPatientRef`)) "None" "SnapToTarget" "SnapToTarget" "KeepWorld" true)
  (`/Game/VRTemplate/Blueprints/VRPawn.ShowConversationInstruction` (`self.VRPawnRef`) (`self.PulseOxValue`) true true "")
  (if (and (`self.bPulseOxPlaced`) (`self.bThermometerPlaced`) (`self.bBPCuffPlaced`) (`self.bStethoscopeHeartPlaced`))
    (set `self.CurrentProcedureState` "NewEnumerator0")
    (`/Game/VRTemplate/Blueprints/VRPawn.ShowConversationInstruction` (`self.VRPawnRef`) (`self.PulseOxValue`) false true "")
    (`PrimitiveComponent.SetCollisionEnabled` (`/Game/VRTemplate/Blueprints/VRPawn.InstructionWidget` (`self.VRPawnRef`)) "QueryOnly")
    (`PrimitiveComponent.SetCollisionEnabled` (`/Game/Actors/BP_EnlargedPatient.StaticMesh` (`self.BPEnlargedPatientRef`)) "NoCollision")))

(fn `CompleteThermometerPlacement`
  (params (KitItemReference :type "/Game/Actors/BP_MedKitItem Object Reference"))
  (locals (CurrentPad :type "/Game/Actors/BP_AEDPad Object Reference") (CurrentMedKitItem :type "/Game/Actors/BP_MedKitItem Object Reference"))
  (bind _output_get (set `local.CurrentMedKitItem` KitItemReference))
  (set `/Game/Actors/BP_MedKitItem.bCorrectlyPlaced` true _output_get)
  (`/Game/VRTemplate/Blueprints/VRPawn.ForceReleaseObject` (`self.VRPawnRef`))
  (set `/Game/VRTemplate/Blueprints/GrabComponent.GrabType` "NewEnumerator0" (`/Game/Actors/BP_MedKitItem.GrabComponent` (`local.CurrentMedKitItem`)))
  (`PrimitiveComponent.SetSimulatePhysics` (`/Game/Actors/BP_MedKitItem.StaticMesh` (`local.CurrentMedKitItem`)) false)
  (`SceneComponent.SetVisibility` (`MedKitItem.LabelWidgetComponent` (`local.CurrentMedKitItem`)) false true)
  (set `self.bThermometerPlaced` true)
  (`self.K2_AttachToComponent` (`local.CurrentMedKitItem`) (`/Game/Actors/BP_EnlargedPatient.ThermometerSnapPoint` (`self.BPEnlargedPatientRef`)) "None" "SnapToTarget" "SnapToTarget" "KeepWorld" true)
  (`/Game/VRTemplate/Blueprints/VRPawn.ShowConversationInstruction` (`self.VRPawnRef`) (`self.ThermometerValue`) true true "")
  (if (and (`self.bPulseOxPlaced`) (`self.bThermometerPlaced`) (`self.bBPCuffPlaced`) (`self.bStethoscopeHeartPlaced`))
    (set `self.CurrentProcedureState` "NewEnumerator0")
    (`/Game/VRTemplate/Blueprints/VRPawn.ShowConversationInstruction` (`self.VRPawnRef`) (`self.ThermometerValue`) false true "")
    (`PrimitiveComponent.SetCollisionEnabled` (`/Game/VRTemplate/Blueprints/VRPawn.InstructionWidget` (`self.VRPawnRef`)) "QueryOnly")
    (`PrimitiveComponent.SetCollisionEnabled` (`/Game/Actors/BP_EnlargedPatient.StaticMesh` (`self.BPEnlargedPatientRef`)) "NoCollision")))

(fn `EndProcedure`
  (`SceneComponent.SetVisibility` (`/Game/Actors/BP_MedKit.StaticMesh` (`self.BPMedKitRef`)) false true)
  (`SceneComponent.SetHiddenInGame` (`/Game/Actors/BP_MedKit.StaticMesh` (`self.BPMedKitRef`)) true true)
  (`PrimitiveComponent.SetCollisionEnabled` (`/Game/Actors/BP_MedKit.StaticMesh` (`self.BPMedKitRef`)) "NoCollision")
  (`SceneComponent.SetVisibility` (`/Game/Actors/BP_MedKitItem.StaticMesh` (`self.StethoscopeRef`)) false true)
  (`SceneComponent.SetVisibility` (`MedKitItem.LabelWidgetComponent` (`self.StethoscopeRef`)) false false)
  (`PrimitiveComponent.SetCollisionEnabled` (`/Game/Actors/BP_MedKitItem.StaticMesh` (`self.StethoscopeRef`)) "NoCollision")
  (`SceneComponent.SetVisibility` (`/Game/Actors/BP_MedKitItem.StaticMesh` (`self.PulseOxRef`)) false true)
  (`SceneComponent.SetVisibility` (`MedKitItem.LabelWidgetComponent` (`self.PulseOxRef`)) false true)
  (`PrimitiveComponent.SetCollisionEnabled` (`/Game/Actors/BP_MedKitItem.StaticMesh` (`self.PulseOxRef`)) "NoCollision")
  (`SceneComponent.SetVisibility` (`/Game/Actors/BP_MedKitItem.StaticMesh` (`self.BPCuffRef`)) false true)
  (`SceneComponent.SetVisibility` (`MedKitItem.LabelWidgetComponent` (`self.BPCuffRef`)) false true)
  (`PrimitiveComponent.SetCollisionEnabled` (`/Game/Actors/BP_MedKitItem.StaticMesh` (`self.BPCuffRef`)) "NoCollision")
  (`SceneComponent.SetVisibility` (`/Game/Actors/BP_MedKitItem.StaticMesh` (`self.ThermometerRef`)) false true)
  (`SceneComponent.SetVisibility` (`MedKitItem.LabelWidgetComponent` (`self.ThermometerRef`)) false true)
  (`PrimitiveComponent.SetCollisionEnabled` (`/Game/Actors/BP_MedKitItem.StaticMesh` (`self.ThermometerRef`)) "NoCollision")
  (`SceneComponent.SetHiddenInGame` (`/Game/Actors/BP_EnlargedPatient.StaticMesh` (`self.BPEnlargedPatientRef`)) true false)
  (`SceneComponent.SetVisibility` (`/Game/Actors/BP_EnlargedPatient.StaticMesh` (`self.BPEnlargedPatientRef`)) false false)
  (`PrimitiveComponent.SetCollisionEnabled` (`/Game/Actors/BP_EnlargedPatient.StaticMesh` (`self.BPEnlargedPatientRef`)) "NoCollision")
  (`SceneComponent.SetVisibility` (`/Game/Actors/BP_Patient.PassengerMesh` (`/Game/VRTemplate/Blueprints/VRPawn.BPPatientRef` (`self.VRPawnRef`))) false true)
  (`SceneComponent.SetHiddenInGame` (`/Game/Actors/BP_EnlargedPatient.BPCuffSphere` (`self.BPEnlargedPatientRef`)) true false)
  (`SceneComponent.SetHiddenInGame` (`/Game/Actors/BP_EnlargedPatient.ThermometerSphere` (`self.BPEnlargedPatientRef`)) true false)
  (`SceneComponent.SetHiddenInGame` (`/Game/Actors/BP_EnlargedPatient.PulseOxSphere` (`self.BPEnlargedPatientRef`)) true false)
  (`SceneComponent.SetHiddenInGame` (`/Game/Actors/BP_EnlargedPatient.StethoscopeSphereHeart` (`self.BPEnlargedPatientRef`)) true false)
  (`SceneComponent.SetHiddenInGame` (`/Game/Actors/BP_EnlargedPatient.StethoscopeSphereLungs` (`self.BPEnlargedPatientRef`)) true false)
  (`AudioComponent.Stop` (`self.MedKitProcedureAudioComp`))
  (`SceneComponent.SetVisibility` (`/Game/Actors/BP_Patient.PassengerMesh` (`/Game/VRTemplate/Blueprints/VRPawn.BPPatientRef` (`self.VRPawnRef`))) true true)
  (set `self.bProcedureActive` false)
  (`/Game/Utility/BP_ConversationComponent.CompletePendingAction` (`/Game/Actors/BP_Patient.BP_ConversationComponent` (`/Game/VRTemplate/Blueprints/VRPawn.BPPatientRef` (`self.VRPawnRef`)))))

(fn `RestoreProcedureDisplay`
  ; display ok button/no shock indicated
  (if (and (`self.bFrontPadPlaced`) (`self.bBackPadPlaced`) (`self.bAEDPoweredOn`))
    (`/Game/VRTemplate/Blueprints/VRPawn.ShowConversationInstruction` (`self.VRPawnRef`) (`self.AEDNoShock`) true true "")
    (else
      ; Power on the AED
      (if (and (`self.bFrontPadPlaced`) (`self.bBackPadPlaced`))
        (`/Game/VRTemplate/Blueprints/VRPawn.ShowConversationInstruction` (`self.VRPawnRef`) (`self.VitalsCompleteInstructionText`) true true "")
        (else
          ; place the pads
          (`/Game/VRTemplate/Blueprints/VRPawn.ShowConversationInstruction` (`self.VRPawnRef`) (`self.ExamAttachItems`) true true ""))))))

(fn `SetUpExam`
  (params (RequestingConversationComponent :type "/Game/Utility/BP_ConversationComponent Object Reference"))
  (bind _pulseoxref (`self.PulseOxRef`))
  (bind _thermometerref (`self.ThermometerRef`))
  (bind _bpcuffref (`self.BPCuffRef`))
  (bind _stethoscoperef (`self.StethoscopeRef`))
  (bind _medkitfloorpoint (`self.MedKitFloorPoint`))
  ; can get rid of input for this and start procedure
  (`/Game/VRTemplate/Blueprints/VRPawn.ForceReleaseObject` (`self.VRPawnRef`))
  (set `/Game/VRTemplate/Blueprints/GrabComponent.GrabType` "NewEnumerator0" (`/Game/Actors/BP_MedKit.GrabComponent` (`self.BPMedKitRef`)))
  (`PrimitiveComponent.SetSimulatePhysics` (`/Game/Actors/BP_MedKit.StaticMesh` (`self.BPMedKitRef`)) false)
  (`self.K2_SetActorLocation` (`self.BPMedKitRef`) (`SceneComponent.K2_GetComponentLocation` _medkitfloorpoint) false true)
  (`self.K2_SetActorRotation` (`self.BPMedKitRef`) (`SceneComponent.K2_GetComponentRotation` _medkitfloorpoint) false)
  (`SceneComponent.SetVisibility` (`/Game/Actors/BP_MedKitItem.StaticMesh` (`self.StethoscopeRef`)) true true)
  (`SceneComponent.SetVisibility` (`MedKitItem.LabelWidgetComponent` (`self.StethoscopeRef`)) true false)
  (set `/Game/Actors/BP_MedKitItem.HomeTransform` (`self.GetTransform` _stethoscoperef) _stethoscoperef)
  (`SceneComponent.SetVisibility` (`/Game/Actors/BP_MedKitItem.StaticMesh` (`self.PulseOxRef`)) true true)
  (`SceneComponent.SetVisibility` (`MedKitItem.LabelWidgetComponent` (`self.PulseOxRef`)) true true)
  (set `/Game/Actors/BP_MedKitItem.HomeTransform` (`self.GetTransform` _pulseoxref) _pulseoxref)
  (`SceneComponent.SetVisibility` (`/Game/Actors/BP_MedKitItem.StaticMesh` (`self.BPCuffRef`)) true true)
  (`SceneComponent.SetVisibility` (`MedKitItem.LabelWidgetComponent` (`self.BPCuffRef`)) true true)
  (set `/Game/Actors/BP_MedKitItem.HomeTransform` (`self.GetTransform` _bpcuffref) _bpcuffref)
  (`SceneComponent.SetVisibility` (`/Game/Actors/BP_MedKitItem.StaticMesh` (`self.ThermometerRef`)) true true)
  (`SceneComponent.SetVisibility` (`MedKitItem.LabelWidgetComponent` (`self.ThermometerRef`)) true true)
  (set `/Game/Actors/BP_MedKitItem.HomeTransform` (`self.GetTransform` _thermometerref) _thermometerref))

(fn `StartProcedure`
  (params (RequestingConversationComponent :type "/Game/Utility/BP_ConversationComponent Object Reference"))
  (bind _output_get (set `self.RequestingConversationComponent` RequestingConversationComponent))
  (`self.SetUpExam` _output_get)
  (set `self.bProcedureActive` true)
  (`/Game/VRTemplate/Blueprints/VRPawn.ShowConversationInstruction` (`self.VRPawnRef`) (`self.ExamAttachItems`) true true "")
  (`SceneComponent.SetVisibility` (`/Game/Actors/BP_Patient.PassengerMesh` (`/Game/VRTemplate/Blueprints/VRPawn.BPPatientRef` (`self.VRPawnRef`))) false true)
  (`SceneComponent.SetVisibility` (`/Game/Actors/BP_EnlargedPatient.StaticMesh` (`self.BPEnlargedPatientRef`)) true false)
  (`PrimitiveComponent.SetCollisionEnabled` (`/Game/Actors/BP_EnlargedPatient.StaticMesh` (`self.BPEnlargedPatientRef`)) "QueryAndPhysics")
  (`SceneComponent.SetHiddenInGame` (`/Game/Actors/BP_EnlargedPatient.BPCuffSphere` (`self.BPEnlargedPatientRef`)) false false)
  (`SceneComponent.SetHiddenInGame` (`/Game/Actors/BP_EnlargedPatient.ThermometerSphere` (`self.BPEnlargedPatientRef`)) false false)
  (`SceneComponent.SetHiddenInGame` (`/Game/Actors/BP_EnlargedPatient.PulseOxSphere` (`self.BPEnlargedPatientRef`)) false false)
  (`SceneComponent.SetHiddenInGame` (`/Game/Actors/BP_EnlargedPatient.StethoscopeSphereHeart` (`self.BPEnlargedPatientRef`)) false false)
  (`SceneComponent.SetHiddenInGame` (`/Game/Actors/BP_EnlargedPatient.StethoscopeSphereLungs` (`self.BPEnlargedPatientRef`)) false false))

(fn `UserConstructionScript`)