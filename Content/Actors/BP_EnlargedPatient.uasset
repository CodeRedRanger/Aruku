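; Enlarged patient model, hidden at BeginPlay, with drop targets for placing AED pads and exam tools (pulse oximeter, thermometer, BP cuff, stethoscope).
; Target overlaps match the actor against references on the AED or exam procedure, then play applause and report completed placement to that procedure.
; Only swapped AED pads trigger booing, once per overlap via a flag cleared on exit.
; Show restores mesh visibility only, while Hide also disables the mesh's collision.
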(event `self.ReceiveBeginPlay`
  (`self.HideEnlargedPatient`))

(event `self.FrontPadTarget.OnComponentBeginOverlap`
  (params (OverlappedComponent :type "PrimitiveComponent Object Reference") (OtherActor :type "Actor Object Reference") (OtherComp :type "PrimitiveComponent Object Reference") (OtherBodyIndex :type Integer) (bFromSweep :type Boolean) (SweepResult :type "HitResult Structure (by ref)"))
  (bind _aedprocedureref (`self.AEDProcedureRef`))
  (bind _frontpadref (`/Game/Actors/BP_AEDProcedure.FrontPadRef` _aedprocedureref))
  (bind _backpadref (`/Game/Actors/BP_AEDProcedure.BackPadRef` (`self.AEDProcedureRef`)))
  (`/Engine/EditorBlueprintResources/StandardMacros.IsValid` _aedprocedureref
    (:`Is Valid`
      (if (== _frontpadref OtherActor)
        (if (not (`/Game/Actors/BP_AEDPad.bCorrectlyPlaced` _frontpadref))
          (`GameplayStatics.PlaySound2D` "/Game/Assets/Audio/SFX/applause.applause" 1.0 1.0 0.0 null null)
          (`/Game/Actors/BP_AEDProcedure.CompleteFrontPadPlacement` (`self.AEDProcedureRef`) _frontpadref))
        (elif (== _backpadref OtherActor)
          (if (not (`/Game/Actors/BP_AEDPad.bWrongPlacementFeedbackPlayed` _backpadref))
            (`GameplayStatics.PlaySound2D` "/Game/Assets/Audio/SFX/booing.booing" 1.0 1.0 0.0 null null)
            (set `/Game/Actors/BP_AEDPad.bWrongPlacementFeedbackPlayed` true _backpadref)))))))

(event `self.BackPadTarget.OnComponentBeginOverlap`
  (params (OverlappedComponent :type "PrimitiveComponent Object Reference") (OtherActor :type "Actor Object Reference") (OtherComp :type "PrimitiveComponent Object Reference") (OtherBodyIndex :type Integer) (bFromSweep :type Boolean) (SweepResult :type "HitResult Structure (by ref)"))
  (bind _aedprocedureref (`self.AEDProcedureRef`))
  (bind _frontpadref (`/Game/Actors/BP_AEDProcedure.FrontPadRef` (`self.AEDProcedureRef`)))
  (bind _backpadref (`/Game/Actors/BP_AEDProcedure.BackPadRef` _aedprocedureref))
  (`/Engine/EditorBlueprintResources/StandardMacros.IsValid` _aedprocedureref
    (:`Is Valid`
      (if (== OtherActor _backpadref)
        (if (not (`/Game/Actors/BP_AEDPad.bCorrectlyPlaced` _backpadref))
          (`GameplayStatics.PlaySound2D` "/Game/Assets/Audio/SFX/applause.applause" 1.0 1.0 0.0 null null)
          (`/Game/Actors/BP_AEDProcedure.CompleteBackPadPlacement` (`self.AEDProcedureRef`) _backpadref))
        (elif (== OtherActor _frontpadref)
          (if (not (`/Game/Actors/BP_AEDPad.bWrongPlacementFeedbackPlayed` _frontpadref))
            (`GameplayStatics.PlaySound2D` "/Game/Assets/Audio/SFX/booing.booing" 1.0 1.0 0.0 null null)
            (set `/Game/Actors/BP_AEDPad.bWrongPlacementFeedbackPlayed` true _frontpadref)))))))

(event `self.FrontPadTarget.OnComponentEndOverlap`
  (params (OverlappedComponent :type "PrimitiveComponent Object Reference") (OtherActor :type "Actor Object Reference") (OtherComp :type "PrimitiveComponent Object Reference") (OtherBodyIndex :type Integer))
  (bind _aedprocedureref (`self.AEDProcedureRef`))
  (bind _backpadref (`/Game/Actors/BP_AEDProcedure.BackPadRef` (`self.AEDProcedureRef`)))
  (`/Engine/EditorBlueprintResources/StandardMacros.IsValid` _aedprocedureref
    (:`Is Valid`
      (if (== (`/Game/Actors/BP_AEDProcedure.FrontPadRef` _aedprocedureref) OtherActor)
        _
        (elif (== _backpadref OtherActor)
          (set `/Game/Actors/BP_AEDPad.bWrongPlacementFeedbackPlayed` false _backpadref))))))

(event `self.BackPadTarget.OnComponentEndOverlap`
  (params (OverlappedComponent :type "PrimitiveComponent Object Reference") (OtherActor :type "Actor Object Reference") (OtherComp :type "PrimitiveComponent Object Reference") (OtherBodyIndex :type Integer))
  (bind _aedprocedureref (`self.AEDProcedureRef`))
  (bind _frontpadref (`/Game/Actors/BP_AEDProcedure.FrontPadRef` (`self.AEDProcedureRef`)))
  (`/Engine/EditorBlueprintResources/StandardMacros.IsValid` _aedprocedureref
    (:`Is Valid`
      (if (== OtherActor (`/Game/Actors/BP_AEDProcedure.BackPadRef` _aedprocedureref))
        _
        (elif (== OtherActor _frontpadref)
          (set `/Game/Actors/BP_AEDPad.bWrongPlacementFeedbackPlayed` false _frontpadref))))))

(event `self.PulseOxTarget.OnComponentBeginOverlap`
  (params (OverlappedComponent :type "PrimitiveComponent Object Reference") (OtherActor :type "Actor Object Reference") (OtherComp :type "PrimitiveComponent Object Reference") (OtherBodyIndex :type Integer) (bFromSweep :type Boolean) (SweepResult :type "HitResult Structure (by ref)"))
  (bind _examprocedureref (`self.ExamProcedureRef`))
  (bind _pulseoxref (`/Game/Actors/BP_ExamProcedure.PulseOxRef` _examprocedureref))
  (`/Engine/EditorBlueprintResources/StandardMacros.IsValid` _examprocedureref
    (:`Is Valid`
      (if (== _pulseoxref OtherActor)
        (if (not (`/Game/Actors/BP_MedKitItem.bCorrectlyPlaced` _pulseoxref))
          (`GameplayStatics.PlaySound2D` "/Game/Assets/Audio/SFX/applause.applause" 1.0 1.0 0.0 null null)
          (`/Game/Actors/BP_ExamProcedure.CompletePulseOxPlacement` (`self.ExamProcedureRef`) _pulseoxref))))))

(event `self.PulseOxTarget.OnComponentEndOverlap`
  (params (OverlappedComponent :type "PrimitiveComponent Object Reference") (OtherActor :type "Actor Object Reference") (OtherComp :type "PrimitiveComponent Object Reference") (OtherBodyIndex :type Integer))
  (`/Engine/EditorBlueprintResources/StandardMacros.IsValid` (`self.ExamProcedureRef`)
    (:`Is Valid`
      (if (== OtherActor (`/Game/Actors/BP_ExamProcedure.PulseOxRef` (`self.ExamProcedureRef`)))
        (set `/Game/Actors/BP_MedKitItem.bWrongPlacementFeedbackPlayed` false (`/Game/Actors/BP_ExamProcedure.PulseOxRef` (`self.ExamProcedureRef`)))))))

(event `self.ThermometerTarget.OnComponentBeginOverlap`
  (params (OverlappedComponent :type "PrimitiveComponent Object Reference") (OtherActor :type "Actor Object Reference") (OtherComp :type "PrimitiveComponent Object Reference") (OtherBodyIndex :type Integer) (bFromSweep :type Boolean) (SweepResult :type "HitResult Structure (by ref)"))
  (bind _thermometerref (`/Game/Actors/BP_ExamProcedure.ThermometerRef` (`self.ExamProcedureRef`)))
  (`/Engine/EditorBlueprintResources/StandardMacros.IsValid` (`self.ExamProcedureRef`)
    (:`Is Valid`
      (if (== OtherActor _thermometerref)
        (if (not (`/Game/Actors/BP_MedKitItem.bCorrectlyPlaced` _thermometerref))
          (`GameplayStatics.PlaySound2D` "/Game/Assets/Audio/SFX/applause.applause" 1.0 1.0 0.0 null null)
          (`/Game/Actors/BP_ExamProcedure.CompleteThermometerPlacement` (`self.ExamProcedureRef`) _thermometerref))))))

(event `self.ThermometerTarget.OnComponentEndOverlap`
  (params (OverlappedComponent :type "PrimitiveComponent Object Reference") (OtherActor :type "Actor Object Reference") (OtherComp :type "PrimitiveComponent Object Reference") (OtherBodyIndex :type Integer))
  (`/Engine/EditorBlueprintResources/StandardMacros.IsValid` (`self.ExamProcedureRef`)
    (:`Is Valid`
      (if (== OtherActor (`/Game/Actors/BP_ExamProcedure.ThermometerRef` (`self.ExamProcedureRef`)))
        (set `/Game/Actors/BP_MedKitItem.bWrongPlacementFeedbackPlayed` false (`/Game/Actors/BP_ExamProcedure.ThermometerRef` (`self.ExamProcedureRef`)))))))

(event `self.BPCuffTarget.OnComponentBeginOverlap`
  (params (OverlappedComponent :type "PrimitiveComponent Object Reference") (OtherActor :type "Actor Object Reference") (OtherComp :type "PrimitiveComponent Object Reference") (OtherBodyIndex :type Integer) (bFromSweep :type Boolean) (SweepResult :type "HitResult Structure (by ref)"))
  (bind _bpcuffref (`/Game/Actors/BP_ExamProcedure.BPCuffRef` (`self.ExamProcedureRef`)))
  (`/Engine/EditorBlueprintResources/StandardMacros.IsValid` (`self.ExamProcedureRef`)
    (:`Is Valid`
      (if (== OtherActor _bpcuffref)
        (if (not (`/Game/Actors/BP_MedKitItem.bCorrectlyPlaced` _bpcuffref))
          (`GameplayStatics.PlaySound2D` "/Game/Assets/Audio/SFX/applause.applause" 1.0 1.0 0.0 null null)
          (`/Game/Actors/BP_ExamProcedure.CompleteBPCuffPlacement` (`self.ExamProcedureRef`) _bpcuffref))))))

(event `self.BPCuffTarget.OnComponentEndOverlap`
  (params (OverlappedComponent :type "PrimitiveComponent Object Reference") (OtherActor :type "Actor Object Reference") (OtherComp :type "PrimitiveComponent Object Reference") (OtherBodyIndex :type Integer))
  (`/Engine/EditorBlueprintResources/StandardMacros.IsValid` (`self.ExamProcedureRef`)
    (:`Is Valid`
      (if (== OtherActor (`/Game/Actors/BP_ExamProcedure.BPCuffRef` (`self.ExamProcedureRef`)))
        (set `/Game/Actors/BP_MedKitItem.bWrongPlacementFeedbackPlayed` false (`/Game/Actors/BP_ExamProcedure.BPCuffRef` (`self.ExamProcedureRef`)))))))

(event `self.StethoscopeHeartTarget.OnComponentBeginOverlap`
  (params (OverlappedComponent :type "PrimitiveComponent Object Reference") (OtherActor :type "Actor Object Reference") (OtherComp :type "PrimitiveComponent Object Reference") (OtherBodyIndex :type Integer) (bFromSweep :type Boolean) (SweepResult :type "HitResult Structure (by ref)"))
  (bind _stethoscoperef (`/Game/Actors/BP_ExamProcedure.StethoscopeRef` (`self.ExamProcedureRef`)))
  (`/Engine/EditorBlueprintResources/StandardMacros.IsValid` (`self.ExamProcedureRef`)
    (:`Is Valid`
      (if (== OtherActor _stethoscoperef)
        (if (not (`/Game/Actors/BP_MedKitItem.bCorrectlyPlaced` _stethoscoperef))
          (`GameplayStatics.PlaySound2D` "/Game/Assets/Audio/SFX/applause.applause" 1.0 1.0 0.0 null null)
          (`/Game/Actors/BP_ExamProcedure.CompleteHeartStethoscopePlacement` (`self.ExamProcedureRef`) _stethoscoperef))))))

(event `self.StethoscopeHeartTarget.OnComponentEndOverlap`
  (params (OverlappedComponent :type "PrimitiveComponent Object Reference") (OtherActor :type "Actor Object Reference") (OtherComp :type "PrimitiveComponent Object Reference") (OtherBodyIndex :type Integer))
  (`/Engine/EditorBlueprintResources/StandardMacros.IsValid` (`self.ExamProcedureRef`)
    (:`Is Valid`
      (if (== OtherActor (`/Game/Actors/BP_ExamProcedure.StethoscopeRef` (`self.ExamProcedureRef`)))
        (set `/Game/Actors/BP_MedKitItem.bWrongPlacementFeedbackPlayed` false (`/Game/Actors/BP_ExamProcedure.StethoscopeRef` (`self.ExamProcedureRef`)))))))

(fn `HideEnlargedPatient`
  (`SceneComponent.SetVisibility` (`self.StaticMesh`) false true)
  (`PrimitiveComponent.SetCollisionEnabled` (`self.StaticMesh`) "NoCollision"))

(fn `ShowEnlargedPatient`
  (`SceneComponent.SetVisibility` (`self.StaticMesh`) true true))

(fn `UserConstructionScript`)