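; BP_CreditsPanel is an actor that hosts the credits screen through a widget component.
; On BeginPlay it hides the component, disables its collision, caches the WBP_Credits widget and binds an event to its return-click callback.
; HandleReturnButtonClicked hides the panel and disables collision; nothing in this file shows it.
; An unconnected fragment would set the VR pawn's active menu state but never runs.
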(event `self.ReceiveBeginPlay`
  (`SceneComponent.SetVisibility` (`self.Widget`) false false)
  (`SceneComponent.SetHiddenInGame` (`self.Widget`) true false)
  (`PrimitiveComponent.SetCollisionEnabled` (`self.Widget`) "NoCollision")
  (bind _aswbp_credits (cast `/Game/Widgets/WBP_Credits` (`WidgetComponent.GetUserWidgetObject` (`self.Widget`))))
  (bind _output_get (set `self. WBP Credits` _aswbp_credits))
  (add `/Game/Widgets/WBP_Credits.OnReturnClicked` _output_get (`|CreateDelegate` :!event `HandleReturnButtonClicked`)))

(fn `HandleReturnButtonClicked`
  (`SceneComponent.SetVisibility` (`self.Widget`) false false)
  (`PrimitiveComponent.SetCollisionEnabled` (`self.Widget`) "NoCollision"))

(fn `UserConstructionScript`)