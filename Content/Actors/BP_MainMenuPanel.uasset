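; VR main menu panel actor that hosts WBP_MainMenu and handles its start, quit, options, credits and high-score reset buttons.
; On BeginPlay it registers with the game instance, puts the VR pawn into menu interaction, hides pawn menus and plays music.
; Options and credits reveal separate panel actors, with options crossfading the music.
; A StartClicked flag blocks quit, options and credits once level start begins.
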(event `self.ReceiveBeginPlay`
  (bind _vrpawn (`self.VRPawn`))
  (bind _vrpawn_2 (`self.VRPawn`))
  (bind _output_get (set `self.MainMenuAudioCompRef` (`self.MainMenuScreenAudioComp`)))
  (set `/Game/Actors/BP_OptionsPanel.MainMenuAudioCompRef` _output_get (`self.BPOptionsPanel`))
  (`AudioComponent.SetSound` (`self.MainMenuScreenAudioComp`) (`self.MainMenuMusic`))
  (bind _output_get_2 (set `self.OptionsMenuAudioCompRef` (`self.OptionsScreenAudioComp`)))
  (set `/Game/Actors/BP_OptionsPanel.OptionsMenuAudioCompRef` _output_get_2 (`self.BPOptionsPanel`))
  (`AudioComponent.SetSound` (`self.OptionsScreenAudioComp`) (`self.OptionsMenuMusic`))
  (bind _asbp_med_game_instance (cast `/Game/Utility/BP_MedGameInstance` (`GameplayStatics.GetGameInstance`)))
  (bind _output_get_3 (set `self.BP Med Game Instance` _asbp_med_game_instance))
  (set `/Game/Utility/BP_MedGameInstance.MainMenuPanelRef` self _output_get_3)
  (bind _asvrpawn (cast `/Game/VRTemplate/Blueprints/VRPawn` (`GameplayStatics.GetPlayerPawn` 0)))
  (bind _output_get_4 (set `self.VRPawn` _asvrpawn))
  (`/Game/VRTemplate/Blueprints/VRPawn.SetMenuInteractionEnabled` _output_get_4 true)
  (`SceneComponent.SetVisibility` (`/Game/VRTemplate/Blueprints/VRPawn.PlayerPauseMenuWidget` (`self.VRPawn`)) false false)
  (`PrimitiveComponent.SetCollisionEnabled` (`/Game/VRTemplate/Blueprints/VRPawn.PlayerPauseMenuWidget` _vrpawn) "NoCollision")
  (`SceneComponent.SetHiddenInGame` (`/Game/VRTemplate/Blueprints/VRPawn.PlayerPauseMenuWidget` (`self.VRPawn`)) true false)
  (set `/Game/VRTemplate/Blueprints/VRPawn.ActiveMenuState` "NewEnumerator1" _vrpawn)
  (bind _aswbp_main_menu (cast `/Game/Widgets/WBP_MainMenu` (`WidgetComponent.GetUserWidgetObject` (`self.Widget`))))
  (bind _output_get_5 (set `self.WBP Main Menu` _aswbp_main_menu))
  (add `/Game/Widgets/WBP_MainMenu.OnStartClicked` _output_get_5 (`|CreateDelegate` :!event `HandleStartClick`))
  (add `/Game/Widgets/WBP_MainMenu.OnQuitClicked` (`self.WBP Main Menu`) (`|CreateDelegate` :!event `HandleQuitClick`))
  (add `/Game/Widgets/WBP_MainMenu.OnOptionsClicked` (`self.WBP Main Menu`) (`|CreateDelegate` :!event `HandleOptionsClick`))
  (add `/Game/Widgets/WBP_MainMenu.OnCreditsClicked` (`self.WBP Main Menu`) (`|CreateDelegate` :!event `HandleCreditsClick`))
  (add `/Game/Widgets/WBP_MainMenu.OnResetOutcomeButton` (`self.WBP Main Menu`) (`|CreateDelegate` :!event `HandleResetOutcomeClick`))
  (add `/Game/Widgets/WBP_MainMenu.OnStartClickStarted` (`self.WBP Main Menu`) (`|CreateDelegate` :!event `HandleStartClickStarted`))
  (`SceneComponent.SetVisibility` (`/Game/VRTemplate/Blueprints/VRPawn.ControlsWReturnWidget` _vrpawn_2) false false)
  (`SceneComponent.SetVisibility` (`/Game/VRTemplate/Blueprints/VRPawn.ControlsWReturnWidget` (`self.VRPawn`)) false false)
  (`PrimitiveComponent.SetCollisionEnabled` (`/Game/VRTemplate/Blueprints/VRPawn.ControlsWReturnWidget` _vrpawn_2) "NoCollision")
  (`SceneComponent.SetVisibility` (`/Game/VRTemplate/Blueprints/VRPawn.OptionsMenuWidget` _vrpawn_2) false false)
  (`SceneComponent.SetVisibility` (`/Game/VRTemplate/Blueprints/VRPawn.OptionsMenuWidget` (`self.VRPawn`)) false false)
  (`PrimitiveComponent.SetCollisionEnabled` (`/Game/VRTemplate/Blueprints/VRPawn.OptionsMenuWidget` _vrpawn_2) "NoCollision")
  (`SceneComponent.SetVisibility` (`/Game/VRTemplate/Blueprints/VRPawn.GraphicsWidget` (`self.VRPawn`)) false false)
  (`SceneComponent.SetHiddenInGame` (`/Game/VRTemplate/Blueprints/VRPawn.GraphicsWidget` (`self.VRPawn`)) true false)
  (`PrimitiveComponent.SetCollisionEnabled` (`/Game/VRTemplate/Blueprints/VRPawn.GraphicsWidget` (`self.VRPawn`)) "NoCollision")
  (`SceneComponent.SetVisibility` (`/Game/VRTemplate/Blueprints/VRPawn.SoundWidget` (`self.VRPawn`)) false false)
  (`SceneComponent.SetHiddenInGame` (`/Game/VRTemplate/Blueprints/VRPawn.SoundWidget` (`self.VRPawn`)) true false)
  (`PrimitiveComponent.SetCollisionEnabled` (`/Game/VRTemplate/Blueprints/VRPawn.SoundWidget` (`self.VRPawn`)) "NoCollision")
  (`AudioComponent.Play` (`self.MainMenuAudioCompRef`) 0.0)
  (set `/Game/Utility/BP_MedGameInstance.LoadingMainMenu` false (`self.BP Med Game Instance`)))

(fn `HandleCreditsClick`
  (if (not (`self.bStartClicked`))
    (`SceneComponent.SetVisibility` (`/Game/Actors/BP_CreditsPanel.Widget` (`self.BPCreditsPanel`)) true false)
    (`PrimitiveComponent.SetCollisionEnabled` (`/Game/Actors/BP_CreditsPanel.Widget` (`self.BPCreditsPanel`)) "QueryOnly")
    (`SceneComponent.SetHiddenInGame` (`/Game/Actors/BP_CreditsPanel.Widget` (`self.BPCreditsPanel`)) false false)))

(fn `HandleOptionsClick`
  (if (not (`self.bStartClicked`))
    (`AudioComponent.FadeOut` (`self.MainMenuAudioCompRef`) 1.0 0.0 "Linear")
    (`AudioComponent.FadeIn` (`self.OptionsMenuAudioCompRef`) 1.0 1.0 0.0 "Linear")
    (`SceneComponent.SetVisibility` (`/Game/Actors/BP_OptionsPanel.Widget` (`self.BPOptionsPanel`)) true false)
    (`PrimitiveComponent.SetCollisionEnabled` (`/Game/Actors/BP_OptionsPanel.Widget` (`self.BPOptionsPanel`)) "QueryOnly")
    (`SceneComponent.SetHiddenInGame` (`/Game/Actors/BP_OptionsPanel.Widget` (`self.BPOptionsPanel`)) false false)))

(fn `HandleQuitClick`
  (if (not (`self.bStartClicked`))
    (`KismetSystemLibrary.QuitGame` null "Quit")))

(fn `HandleResetOutcomeClick`
  (bind _asbp_med_game_instance (cast `/Game/Utility/BP_MedGameInstance` (`GameplayStatics.GetGameInstance`)))
  (set `/Game/Utility/BP_MedGameInstance.SavedHighScoreLevel1` 0.0 _asbp_med_game_instance)
  (`/Game/Utility/BP_MedGameInstance.SaveSettings` _asbp_med_game_instance)
  (`/Game/Widgets/WBP_MainMenu.UpdateHighScorePercent` (`self.WBP Main Menu`)))

(fn `HandleStartClick`
  (set `/Game/VRTemplate/Blueprints/VRPawn.ActiveMenuState` "NewEnumerator0" (`self.VRPawn`))
  (`/Game/VRTemplate/Blueprints/VRPawn.SetMenuInteractionEnabled` (`self.VRPawn`) false)
  (set `/Game/Utility/BP_MedGameInstance.CurrentScenarioLevel` (`/Game/Widgets/WBP_MainMenu.Level Name` (`self.WBP Main Menu`)) (`self.BP Med Game Instance`))
  (`GameplayStatics.OpenLevel` (`/Game/Widgets/WBP_MainMenu.Level Name` (`self.WBP Main Menu`))))

(fn `HandleStartClickStarted`
  (set `self.bStartClicked` true))

(fn `UserConstructionScript`)