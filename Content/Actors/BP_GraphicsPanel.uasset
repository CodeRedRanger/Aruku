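; BP_GraphicsPanel is an actor that hosts the WBP_Graphics menu in a widget component, as a graphics panel.
; On BeginPlay it hides the component, disables its collision, caches the user widget and binds to its return-clicked event.
; HandleReturnButtonClicked hides the component and disables collision again; nothing here shows the panel.
; Leftover unwired nodes, including one setting the VRPawn menu state, never run.
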(event `self.ReceiveBeginPlay`
  (`SceneComponent.SetVisibility` (`self.Widget`) false false)
  (`PrimitiveComponent.SetCollisionEnabled` (`self.Widget`) "NoCollision")
  (`SceneComponent.SetHiddenInGame` (`self.Widget`) true false)
  (bind _aswbp_graphics (cast `/Game/Widgets/WBP_Graphics` (`WidgetComponent.GetUserWidgetObject` (`self.Widget`))))
  (bind _output_get (set `self.WBP Graphics` _aswbp_graphics))
  (add `/Game/Widgets/WBP_Graphics.OnReturnClicked` _output_get (`|CreateDelegate` :!event `HandleReturnButtonClicked`)))

(fn `HandleReturnButtonClicked`
  (`SceneComponent.SetVisibility` (`self.Widget`) false false)
  (`PrimitiveComponent.SetCollisionEnabled` (`self.Widget`) "NoCollision"))

(fn `UserConstructionScript`)