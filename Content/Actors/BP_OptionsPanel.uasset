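; VR options menu panel actor that hosts a WBP_OptionsMenu widget and opens the sound, graphics and control sub-panels.
; On BeginPlay it hides the widget, disables its collision, binds the menu's button events and sets the VRPawn's active menu state.
; Option clicks reveal the matching panel actor and enable its query collision.
; Return hides this panel, crossfades from options to main menu audio and updates the pawn's menu state.
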(event `self.ReceiveBeginPlay`
  (bind _asvrpawn (cast `/Game/VRTemplate/Blueprints/VRPawn` (`GameplayStatics.GetPlayerPawn` 0)))
  (set `self.VRPawn` _asvrpawn)
  (`SceneComponent.SetVisibility` (`self.Widget`) false false)
  (`SceneComponent.SetHiddenInGame` (`self.Widget`) true false)
  (`PrimitiveComponent.SetCollisionEnabled` (`self.Widget`) "NoCollision")
  (bind _aswbp_options_menu (cast `/Game/Widgets/WBP_OptionsMenu` (`WidgetComponent.GetUserWidgetObject` (`self.Widget`))))
  (bind _output_get (set `self.WBP Option Menu` _aswbp_options_menu))
  (add `/Game/Widgets/WBP_OptionsMenu.OnSoundOptionsClicked` _output_get (`|CreateDelegate` :!event `HandleSoundOptionsClicked`))
  (add `/Game/Widgets/WBP_OptionsMenu.OnGraphicsOptionsClicked` (`self.WBP Option Menu`) (`|CreateDelegate` :!event `HandleGraphicsOptionsClicked`))
  (add `/Game/Widgets/WBP_OptionsMenu.OnControlOptionsClicked` (`self.WBP Option Menu`) (`|CreateDelegate` :!event `HandleControlOptionsClicked`))
  (add `/Game/Widgets/WBP_OptionsMenu.OnReturnButtonClicked` (`self.WBP Option Menu`) (`|CreateDelegate` :!event `HandleReturnButtonClicked`))
  (set `/Game/VRTemplate/Blueprints/VRPawn.ActiveMenuState` "NewEnumerator6" (`self.VRPawn`)))

(fn `HandleControlOptionsClicked`
  (`SceneComponent.SetVisibility` (`/Game/Actors/BP_ControlsPanel.Widget` (`self.BPControlPanel`)) true false)
  (`PrimitiveComponent.SetCollisionEnabled` (`/Game/Actors/BP_ControlsPanel.Widget` (`self.BPControlPanel`)) "QueryOnly")
  (`SceneComponent.SetVisibility` (`/Game/Actors/BP_ControlsPanel.DefaultSceneRoot` (`self.BPControlPanel`)) true false)
  (`SceneComponent.SetHiddenInGame` (`/Game/Actors/BP_ControlsPanel.Widget` (`self.BPControlPanel`)) false false))

(fn `HandleGraphicsOptionsClicked`
  (`SceneComponent.SetVisibility` (`/Game/Actors/BP_GraphicsPanel.Widget` (`self.BPGraphisPanel`)) true false)
  (`PrimitiveComponent.SetCollisionEnabled` (`/Game/Actors/BP_GraphicsPanel.Widget` (`self.BPGraphisPanel`)) "QueryOnly")
  (`SceneComponent.SetVisibility` (`/Game/Actors/BP_GraphicsPanel.DefaultSceneRoot` (`self.BPGraphisPanel`)) true false)
  (`SceneComponent.SetHiddenInGame` (`/Game/Actors/BP_GraphicsPanel.Widget` (`self.BPGraphisPanel`)) false false))

(fn `HandleReturnButtonClicked`
  (`AudioComponent.FadeOut` (`self.OptionsMenuAudioCompRef`) 1.0 0.0 "Linear")
  (`AudioComponent.FadeIn` (`self.MainMenuAudioCompRef`) 1.0 1.0 0.0 "Linear")
  (`SceneComponent.SetVisibility` (`self.Widget`) false false)
  (`PrimitiveComponent.SetCollisionEnabled` (`self.Widget`) "NoCollision")
  (`SceneComponent.SetHiddenInGame` (`self.Widget`) true false)
  (set `/Game/VRTemplate/Blueprints/VRPawn.ActiveMenuState` "NewEnumerator1" (`self.VRPawn`)))

(fn `HandleSoundOptionsClicked`
  (`SceneComponent.SetVisibility` (`/Game/Actors/BP_SoundPanel.Widget` (`self.BPSoundPanel`)) true false)
  (`PrimitiveComponent.SetCollisionEnabled` (`/Game/Actors/BP_SoundPanel.Widget` (`self.BPSoundPanel`)) "QueryOnly")
  (`SceneComponent.SetVisibility` (`/Game/Actors/BP_SoundPanel.DefaultSceneRoot` (`self.BPSoundPanel`)) true false)
  (`SceneComponent.SetHiddenInGame` (`/Game/Actors/BP_SoundPanel.Widget` (`self.BPSoundPanel`)) false false))

(fn `UserConstructionScript`)