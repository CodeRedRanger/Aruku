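; Water ripple effect actor that plays an expanding, fading ring on a plane mesh.
; On BeginPlay it waits a configurable start delay, then creates a dynamic material instance on the plane.
; A timeline then drives the plane's horizontal scale and the material's RippleOpacity parameter.
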(event `self.ReceiveBeginPlay`
  (`KismetSystemLibrary.Delay` (`self.StartDelay`))
  (bind _returnvalue (`PrimitiveComponent.CreateDynamicMaterialInstance` (`self.Plane`) 0 null "None"))
  (set `self.RippleMat` _returnvalue)
  (bind (_direction _scale _opacity) (`Timeline|TL_Ripple`)
    (:`Update`
      (`SceneComponent.SetRelativeScale3D` (`self.Plane`) (`KismetMathLibrary.MakeVector` _scale _scale 1.0))
      (`MaterialInstanceDynamic.SetScalarParameterValue` (`self.RippleMat`) "RippleOpacity" _opacity))))

(fn `UserConstructionScript`)