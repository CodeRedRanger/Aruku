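; AI dog that plays fetch with a toy and can follow the player.
; On BeginPlay it heads for the first toy found, or destroys itself if the game instance's network state doesn't match.
; Fetch and follow events use looping timers to re-issue navmesh-projected AI moves.
; GrabRange overlap attaches the toy to a mouth socket, brings it near the player, turns via timeline, then re-enables toy collision.
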(event `self.ReceiveBeginPlay`
  (bind _asbp_med_game_instance (cast `/Game/Utility/BP_MedGameInstance` (`GameplayStatics.GetGameInstance`)))
  (if (`|EnumEquality` (`/Game/Utility/BP_MedGameInstance.NetworkState` _asbp_med_game_instance) "NewEnumerator0")
    (bind _outactors (`GameplayStatics.GetAllActorsOfClass` "/Game/SB/Dog/bp_toy.bp_toy_C"))
    (`|AIMoveTo` self (0.0 0.0 0.0) (`|GetArrayItem` _outactors))
    (else
      (`self.K2_DestroyActor`))))

(event `self.ReceiveTick`
  (params (DeltaSeconds :type "Float (single-precision)")))

(event `self.GrabRange.OnComponentBeginOverlap`
  (params (OverlappedComponent :type "PrimitiveComponent Object Reference") (OtherActor :type "Actor Object Reference") (OtherComp :type "PrimitiveComponent Object Reference") (OtherBodyIndex :type Integer) (bFromSweep :type Boolean) (SweepResult :type "HitResult Structure (by ref)"))
  (bind _returnvalue (`self.K2_GetActorLocation` (`GameplayStatics.GetPlayerPawn` 0)))
  (bind _asbp_toy (cast `/Game/SB/Dog/bp_toy` OtherActor))
  (`self.DogGrab` _asbp_toy)
  (if (not (< (`self.GetDistanceTo` (`GameplayStatics.GetPlayerPawn` 0)) 100.0))
    (`|AIMoveTo` self (+ _returnvalue (100.0 0.0 0.0)) null 100.0
      (:`OnSuccess`
        _)))
  (bind _output_get (set `self.TurnStartRot` (`self.K2_GetActorRotation`)))
  (bind (_direction _alpha) (`Timeline|TurnToPlayer` :!via `PlayFromStart`)
    (:`Update`
      (`self.K2_SetActorRotation` (`KismetMathLibrary.RLerp` _output_get (`KismetMathLibrary.MakeRotator` 0.0 0.0 (.yaw (`KismetMathLibrary.FindLookAtRotation` (`self.K2_GetActorLocation`) _returnvalue))) _alpha true)))
    (:`Finished`
      (`PrimitiveComponent.SetCollisionEnabled` (`/Game/SB/Dog/bp_toy.ToyMesh` _asbp_toy) "QueryAndPhysics"))))

(event `StartFetch_Event`
  (bind _returnvalue (`KismetSystemLibrary.K2_SetTimerDelegate` (delegate `UpdateFetchTarget_Event`) 0.1 true))
  (set `self.FetchTimerHandle` _returnvalue))

(event `UpdateFetchTarget_Event`
  (`/Engine/EditorBlueprintResources/StandardMacros.IsValid` (`self.FetchToy`)
    (:`Is Valid`
      (`|AIMoveTo` self (`NavigationSystemV1.K2_ProjectPointToNavigation` (`self.K2_GetActorLocation` (`self.FetchToy`))) null))))

(event `StartFollowingPlayer_Event`
  (if (not (`self.IsFollowingPlayer`))
    (set `self.IsFollowingPlayer` true)
    (bind _returnvalue (`KismetSystemLibrary.K2_SetTimerDelegate` (delegate `UpdateFollowTarget_Event`) 0.1 true))
    (set `self.FollowTimerHandle` _returnvalue)))

(event `UpdateFollowTarget_Event`
  (if (`self.IsFollowingPlayer`)
    (`|AIMoveTo` self (`NavigationSystemV1.K2_ProjectPointToNavigation` (`self.K2_GetActorLocation` (`GameplayStatics.GetPlayerPawn` 0))) null 100.0)))

(fn `DogGrab`
  (params (Toy :type "/Game/SB/Dog/bp_toy Object Reference"))
  (bind _grabcomponent (`/Game/SB/Dog/bp_toy.GrabComponent` Toy))
  (bind _toymesh (`/Game/SB/Dog/bp_toy.ToyMesh` Toy))
  (`/Engine/EditorBlueprintResources/StandardMacros.IsValid` Toy
    (:`Is Valid`
      (if (not (`/Game/VRTemplate/Blueprints/GrabComponent.bIsHeld` _grabcomponent))
        (`KismetSystemLibrary.K2_ClearAndInvalidateTimerHandle` (`self.FetchTimerHandle`))
        (set `self.FetchToy` null)
        (`/Engine/EditorBlueprintResources/StandardMacros.IsValid` (`self.FetchToy`)
          (:`Is Not Valid`
            (set `self.FetchToy` Toy)
            (`/Game/VRTemplate/Blueprints/GrabComponent.SetPrimitiveCompPhysics` _grabcomponent false)
            (`PrimitiveComponent.SetCollisionEnabled` _toymesh "NoCollision")
            (bind _returnvalue (`SceneComponent.K2_AttachToComponent` _toymesh (`self.Mesh`) "ToySocket" "SnapToTarget" "SnapToTarget" "KeepWorld" false))
            (if _returnvalue
              (set `self.IsHeldDog` true)
              (`PrimitiveComponent.SetCollisionEnabled` (`self.GrabRange`) "NoCollision")
              (else
                (`/Game/VRTemplate/Blueprints/GrabComponent.SetPrimitiveCompPhysics` _grabcomponent true)
                (`PrimitiveComponent.SetCollisionEnabled` _toymesh "QueryAndPhysics")))))))))

(fn `UserConstructionScript`)