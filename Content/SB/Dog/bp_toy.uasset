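; A grabbable toy that drives a fetch game with the first Bp_dog found in the level.
; Grabbing it clears the dog's held flag and fetch target, then starts the dog following the player.
; Dropping it stops following, sets itself as the fetch target and starts fetch after a short delay.
; The dog's grab range and capsule collision are disabled during that delay, then restored as query-only.
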(event `self.ReceiveBeginPlay`)

(event `self.GrabComponent.OnGrabbed`
  (bind _outactors (`GameplayStatics.GetAllActorsOfClass` "/Game/SB/Dog/bp_dog.bp_dog_C"))
  (bind _output (`|GetArrayItem` _outactors))
  (set `/Game/SB/Dog/bp_dog.IsHeldDog` false _output)
  (set `/Game/SB/Dog/bp_dog.FetchToy` null _output)
  (`/Game/SB/Dog/bp_dog.StartFollowingPlayer_Event` _output))

(event `self.GrabComponent.OnDropped`
  (bind _outactors (`GameplayStatics.GetAllActorsOfClass` "/Game/SB/Dog/bp_dog.bp_dog_C"))
  (bind _output (`|GetArrayItem` _outactors))
  (set `/Game/SB/Dog/bp_dog.IsFollowingPlayer` false _output)
  (`KismetSystemLibrary.K2_ClearAndInvalidateTimerHandle` (`/Game/SB/Dog/bp_dog.FollowTimerHandle` _output))
  (set `/Game/SB/Dog/bp_dog.FetchToy` self _output)
  (`PrimitiveComponent.SetCollisionEnabled` (`/Game/SB/Dog/bp_dog.GrabRange` _output) "NoCollision")
  (`PrimitiveComponent.SetCollisionEnabled` (`Character.CapsuleComponent` _output) "NoCollision")
  (`KismetSystemLibrary.Delay` 0.5)
  (`/Game/SB/Dog/bp_dog.StartFetch_Event` _output)
  (`PrimitiveComponent.SetCollisionEnabled` (`/Game/SB/Dog/bp_dog.GrabRange` _output) "QueryOnly")
  (`PrimitiveComponent.SetCollisionEnabled` (`Character.CapsuleComponent` _output) "QueryOnly"))

(fn `UserConstructionScript`)